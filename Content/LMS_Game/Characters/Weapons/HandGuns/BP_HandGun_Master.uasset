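; BP_HandGun_Master is the handgun master Blueprint, adding a weapon spin effect to whatever its parent provides.
; BeginPlay caches the root component's relative rotation.
; StartSpinWeapon drives RotatingMovement at high speed, pivoting around the mesh's Trigger_Bone socket for a trigger-centred twirl.
; EndSpinWeapon stops the movement, clears the pivot, restores the cached rotation and zeroes the root's relative location.
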(event `self.ReceiveBeginPlay`
  (`parent.ReceiveBeginPlay`)
  (set `self.Relative Rotation` (`SceneComponent.RelativeRotation` (`self.DefaultSceneRoot`))))

(event `self.Start Spin Weapon`
  (bind _rotatingmovement (`self.RotatingMovement`))
  (set `RotatingMovementComponent.PivotTranslation` (.location (`SceneComponent.GetSocketTransform` (`self.Weapon SM`) "Trigger_Bone" "RTS_Component")) _rotatingmovement)
  (set `RotatingMovementComponent.RotationRate` (struct :`Roll` -3000.0) _rotatingmovement))

(event `self.End Spin Weapon`
  (bind _rotatingmovement (`self.RotatingMovement`))
  (bind _defaultsceneroot (`self.DefaultSceneRoot`))
  (`MovementComponent.StopMovementImmediately` _rotatingmovement)
  (set `RotatingMovementComponent.RotationRate` (struct) _rotatingmovement)
  (set `RotatingMovementComponent.PivotTranslation` (0.0 0.0 0.0) (`self.RotatingMovement`))
  (`SceneComponent.K2_SetRelativeRotation` _defaultsceneroot (`self.Relative Rotation`) false false)
  (`SceneComponent.K2_SetRelativeLocation` _defaultsceneroot (0.0 0.0 0.0) false true))

(fn `UserConstructionScript`
  (`parent.UserConstructionScript`))