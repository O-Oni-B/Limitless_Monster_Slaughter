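; BP_Master_PickUp is a pickup, named as a master class, that grants ammo to the character interacting with it.
; The interact event calls AddAmmo, which casts to BP_LMS_BaseCharacter, adds the per-crate amount to its weapon component's ammo map, then destroys the pickup.
; PickUpItem does the same for the item inventory map, reusing the per-crate amount, but is not called here.
; A timed self-destruct is left unconnected.
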(event `self.ReceiveBeginPlay`)

(event `/Game/LMS_Game/Characters/Interfaces/IF_Interact.IF_Interact`
  (params (Interactor :type "Actor Object Reference"))
  (`self.Add Ammo` Interactor))

(fn `Add Ammo`
  (params (Interactor :type "Actor Object Reference"))
  (bind _asbp_lms_base_character (cast `/Game/LMS_Game/Characters/Character_Logic/BP_LMS_BaseCharacter` Interactor))
  (bind _ammo_type___ttl_ammo (`/Game/LMS_Game/Characters/Actor_Components/BPC_Weapon_System.Ammo Type / Ttl Ammo` (`/Game/LMS_Game/Characters/Character_Logic/BP_LMS_BaseCharacter.BPC_Weapon_System` _asbp_lms_base_character)))
  (`BlueprintMapLibrary.Map_Add` _ammo_type___ttl_ammo (`self.Ammo Type`) (+ (`BlueprintMapLibrary.Map_Find` _ammo_type___ttl_ammo (`self.Ammo Type`)) (`self.Ammp Per Crate`)))
  (`self.K2_DestroyActor`))

(fn `Pick Up Item`
  (params (Interactor :type "Actor Object Reference") (`Item Type` :type "/Game/LMS_Game/Characters/Enums/E_Item_Type Enum (by ref)"))
  (bind _asbp_lms_base_character (cast `/Game/LMS_Game/Characters/Character_Logic/BP_LMS_BaseCharacter` Interactor))
  (bind _item_inventory (`/Game/LMS_Game/Characters/Actor_Components/BPC_Weapon_System.Item Inventory` (`/Game/LMS_Game/Characters/Character_Logic/BP_LMS_BaseCharacter.BPC_Weapon_System` _asbp_lms_base_character)))
  (`BlueprintMapLibrary.Map_Add` _item_inventory `Item Type` (+ (`BlueprintMapLibrary.Map_Find` _item_inventory `Item Type`) (`self.Ammp Per Crate`)))
  (`self.K2_DestroyActor`))

(fn `UserConstructionScript`)