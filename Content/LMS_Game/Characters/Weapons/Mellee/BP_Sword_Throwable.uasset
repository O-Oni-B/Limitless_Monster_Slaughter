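; Thrown sword projectile that deals damage on hit and swaps itself for a BP_Sword_10 at the impact point.
; A MeleeTrace line trace along the blade starts shortly after BeginPlay, and its first hit stops movement and applies bone-scaled point damage, favoring head and neck.
; The spawned sword attaches to what was hit, or changes weapon state if that target is dead.
; Tick's sphere trace and the component hit events have no effect.
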(event `self.ReceiveTick`
  (params (DeltaSeconds :type "Float (single-precision)"))
  (if (`self.Is Mid Throw`)
    (bind _outhit (`KismetSystemLibrary.SphereTraceSingle` (`SceneComponent.K2_GetComponentLocation` (`self.Sword Start`)) (`SceneComponent.K2_GetComponentLocation` (`self.Sword End`)) 5.0 "TraceTypeQuery1" false (`|MakeArray` (`self.Throwing Actor`))))
    (if (`GameplayStatics.BreakHitResult` _outhit)
      _)))

(event `self.ReceiveBeginPlay`
  (`KismetSystemLibrary.Delay` 0.1)
  (`PrimitiveComponent.SetCollisionResponseToChannel` (`self.Blade Collision`) "ECC_Pawn" "ECR_Block")
  (`PrimitiveComponent.SetCollisionResponseToChannel` (`self.Sword`) "ECC_Pawn" "ECR_Block")
  (bind _returnvalue (`MeleeTraceComponent.StartTrace` (`self.MeleeTrace`) (make `MeleeTraceInfo` "Sword Start" "Sword End" (`MeleeTraceShape_Line.MakeLineShape`) 10)))
  (set `self.Melee trace Handle` _returnvalue))

(event `self.Sword.OnComponentHit`
  (params (HitComponent :type "PrimitiveComponent Object Reference") (OtherActor :type "Actor Object Reference") (OtherComp :type "PrimitiveComponent Object Reference") (NormalImpulse :type "Vector Structure") (Hit :type "HitResult Structure (by ref)")))

(event `self.Blade Collision.OnComponentHit`
  (params (HitComponent :type "PrimitiveComponent Object Reference") (OtherActor :type "Actor Object Reference") (OtherComp :type "PrimitiveComponent Object Reference") (NormalImpulse :type "Vector Structure") (Hit :type "HitResult Structure (by ref)")))

(event `self.MeleeTrace.OnTraceHit`
  (params (ThisComponent :type "MeleeTraceComponent Object Reference") (HitActor :type "Actor Object Reference") (HitLocation :type "Vector Structure (by ref)") (HitNormal :type "Vector Structure (by ref)") (HitBoneName :type Name))
  (bind (_returnvalue_roll _returnvalue_pitch _returnvalue_yaw) (`KismetMathLibrary.BreakRotator` (`KismetMathLibrary.MakeRotFromZ` HitNormal)))
  (`MovementComponent.StopMovementImmediately` (`self.ProjectileMovement`))
  (set `RotatingMovementComponent.RotationRate` (struct) (`self.RotatingMovement`))
  (set `ProjectileMovementComponent.ProjectileGravityScale` 0.0 (`self.ProjectileMovement`))
  (`GameplayStatics.ApplyPointDamage` HitActor (`self.Get Location Damage Multiplier` HitBoneName 15.0) (`KismetMathLibrary.GetForwardVector` (`KismetMathLibrary.FindLookAtRotation` HitLocation HitNormal)) (`GameplayStatics.MakeHitResult` false false 0.0 0.0 HitLocation (0.0 0.0 0.0) (0.0 0.0 1.0) (0.0 0.0 1.0) null null null HitBoneName) null (`self.Throwing Actor`))
  (set `self.Is Mid Throw` false)
  (bind _returnvalue (`|SpawnActorFromClass` "/Game/LMS_Game/Characters/Weapons/Mellee/BP_Sword_10.BP_Sword_10_C" (`KismetMathLibrary.MakeTransform` (+ HitLocation (* (`KismetMathLibrary.GetForwardVector` (`KismetMathLibrary.MakeRotFromX` HitNormal)) 25.0)) (`KismetMathLibrary.MakeRotator` 100.0 0.0 _returnvalue_yaw)) "AlwaysSpawn" "OverrideRootScale" null "NewEnumerator3" null))
  (bind _actor (message `/Game/LMS_Game/Characters/Interfaces/IF_WeaponOwner_Interface.IF Get Actor References` HitActor))
  (`/Engine/EditorBlueprintResources/StandardMacros.IsValid` _actor
    (:`Is Valid`
      (bind _dead_ (message `/Game/LMS_Game/Characters/Interfaces/IF_WeaponOwner_Interface.IF Is Dead` _actor))
      (if _dead_
        (`/Game/LMS_Game/Characters/Weapons/BP_Weapon_Master.Set Weapon State ` _returnvalue "NewEnumerator0")
        (else
          (`self.K2_AttachToComponent` _returnvalue (`Character.Mesh` _actor) HitBoneName "KeepWorld" "KeepWorld" "SnapToTarget" true))))
    (:`Is Not Valid`
      (`self.K2_AttachToActor` _returnvalue HitActor HitBoneName "KeepWorld" "KeepWorld" "KeepWorld" true)))
  (`self.K2_DestroyActor`))

(fn `Get Location Damage Multiplier`
  (params (`Hit Bone Name` :type Name) (`Base Damage` :type "Float (double-precision)"))
  (returns (`Damage Result` :type "Float (double-precision)") (`Critical Hit Result` :type Boolean))
  (locals (`Local Multiplier` :type "Float (double-precision)") (`Is Critical?` :type Boolean))
  (switch `name` `Hit Bone Name`
    (:`Default`
      (set `local.Local Multiplier` 1.0 :!label _label)
      (set `local.Is Critical?` false))
    (:`pelvis`
      (goto _label))
    (:`spine_01`
      (goto _label))
    (:`spine_02`
      (goto _label))
    (:`spine_03`
      (goto _label))
    (:`spine_04`
      (goto _label))
    (:`spine_05`
      (goto _label))
    (:`clavicle_l`
      (set `local.Local Multiplier` 0.8 :!label _label_2)
      (set `local.Is Critical?` false))
    (:`upperarm_l`
      (set `local.Local Multiplier` 0.7 :!label _label_3)
      (set `local.Is Critical?` false))
    (:`lowerarm_l`
      (goto _label_3))
    (:`hand_l`
      (goto _label_3))
    (:`clavicle_r`
      (goto _label_2))
    (:`upperarm_r`
      (goto _label_3))
    (:`lowerarm_r`
      (goto _label_3))
    (:`hand_r`
      (goto _label_3))
    (:`thigh_l`
      (goto _label_2))
    (:`calf_l`
      (goto _label_3))
    (:`foot_l`
      (goto _label_3))
    (:`thigh_r`
      (goto _label_2))
    (:`calf_r`
      (goto _label_3))
    (:`foot_r`
      (goto _label_3))
    (:`neck_01`
      (set `local.Local Multiplier` 2.0 :!label _label_4)
      (set `local.Is Critical?` true))
    (:`neck_02`
      (goto _label_4))
    (:`head`
      (goto _label_4)))
  (return (* (`local.Base Damage`) (`local.Local Multiplier`)) (`local.Is Critical?`)))

(fn `UserConstructionScript`)