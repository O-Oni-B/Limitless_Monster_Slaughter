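; BP_Grenade is a timed grenade that explodes a few seconds after BeginPlay, then destroys itself.
; The blast spawns a scaled particle effect and loud sound, applies radial damage with falloff, and fires a RadialForce impulse.
; It gets the owner's camera through an interface message and centers a world camera shake on that camera's location rather than on the explosion.
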(event `self.ReceiveBeginPlay`
  (bind _returnvalue (`self.K2_GetActorLocation`))
  (`KismetSystemLibrary.Delay` 3.0)
  (`GameplayStatics.SpawnEmitterAtLocation` "/Game/LMS_Game/Imported_Assets/MilitaryWeapSilver/FX/P_Grenade_Explosion_01.P_Grenade_Explosion_01" _returnvalue (`self.K2_GetActorRotation`) (3.0 3.0 3.0))
  (`GameplayStatics.PlaySoundAtLocation` "/Game/StarterContent/Audio/Explosion_Cue.Explosion_Cue" _returnvalue (struct) 1000.0 1.0 0.0 null null self null)
  (`GameplayStatics.ApplyRadialDamageWithFalloff` :`BaseDamage` 100.0 :`MinimumDamage` 50.0 :`Origin` _returnvalue :`DamageInnerRadius` 400.0 :`DamageOuterRadius` 800.0 :`DamageFalloff` 0.1 :`DamageCauser` self :`InstigatedByController` null :`DamagePreventionChannel` "ECC_Camera")
  (`RadialForceComponent.FireImpulse` (`self.RadialForce`))
  (bind (_actor _actor_camera) (message `/Game/LMS_Game/Characters/Interfaces/IF_WeaponOwner_Interface.IF Get Actor References` (`self.GetOwner`)))
  (`GameplayStatics.PlayWorldCameraShake` "/Game/LMS_Game/Characters/Camera_Mislenious/BP_CameraShake_Finisher.BP_CameraShake_Finisher_C" (`SceneComponent.K2_GetComponentLocation` _actor_camera) 100.0 500.0)
  (`self.K2_DestroyActor`))

(fn `UserConstructionScript`)