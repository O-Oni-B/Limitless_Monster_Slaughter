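; Base weapon actor that can be picked up through the interact interface, handing itself to the interactor's BPC_Weapon_System.
; The construction script loads weapon data from DT_Weapon_Table by WeaponID and randomizes current ammo between half and full magazine.
; SetWeaponState switches collision, physics and attachment for Dropped, Equipped, In Hand and Stabbed states, starting from a default on BeginPlay.
; Player overlap toggles a name prompt widget; spin events are empty stubs.
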(event `self.ReceiveBeginPlay`
  (`self.Set Weapon State ` (`self.Default Weapon State`)))

(event `/Game/LMS_Game/Characters/Interfaces/IF_Interact.IF_Interact`
  (params (Interactor :type "Actor Object Reference"))
  ;[0.05098 0.05098 0.05098] Interact Function - This Interface Function Checks if the interactor has the Weapon System Component in the Interacting Actor and calls the Pick Up Weapon Function and Cast to the Character to get  Character Ref to be called in the future
  (bind _output_get (set `self.Interactor` Interactor))
  (`/Game/LMS_Game/Characters/Actor_Components/BPC_Weapon_System.Pick Up Weapon` (`self.GetComponentByClass` Interactor "/Game/LMS_Game/Characters/Actor_Components/BPC_Weapon_System.BPC_Weapon_System_C") self)
  (bind _ascharacter (cast `Character` _output_get))
  (set `self.Character Ref ` _ascharacter))

(event `self.Interaction Area.OnComponentBeginOverlap`
  (params (OverlappedComponent :type "PrimitiveComponent Object Reference") (OtherActor :type "Actor Object Reference") (OtherComp :type "PrimitiveComponent Object Reference") (OtherBodyIndex :type Integer) (bFromSweep :type Boolean) (SweepResult :type "HitResult Structure (by ref)"))
  (bind _widget (`self.Widget`))
  ;[0.05098 0.05098 0.05098] Activating and Deactivating Interact UI - When Overlaps with specifically BP_Player_Character or Children of this class, The Interact Widget (UI) is activated Showing the Name Of the Weapon Being Overlappeed With, and toggles the Widget's visibility
  (cast `/Game/LMS_Game/Characters/Character_Logic/BP_LMS_PlayerCharacter` OtherActor)
  (set `self.Can Pick ` true)
  (`self.Interact UI`
    (:`then`
      _)
    (:`else`
      (bind _returnvalue (`|CreateWidget` "/Game/LMS_Game/UI/WB_Interact.WB_Interact_C" null (`.WeaponName_2_70B92C3E461952DD4AA8428ED417F3D2` (break `/Game/LMS_Game/Characters/Structures/S_Weapon_Struct` (`self.Weapon_Structure`)))))
      (set `self.Interact UI` _returnvalue)))
  (`WidgetComponent.SetWidget` _widget _returnvalue)
  (`SceneComponent.SetVisibility` _widget true false))

(event `self.Interaction Area.OnComponentEndOverlap`
  (params (OverlappedComponent :type "PrimitiveComponent Object Reference") (OtherActor :type "Actor Object Reference") (OtherComp :type "PrimitiveComponent Object Reference") (OtherBodyIndex :type Integer))
  ;[0.05098 0.05098 0.05098] Activating and Deactivating Interact UI - When Overlaps with specifically BP_Player_Character or Children of this class, The Interact Widget (UI) is activated Showing the Name Of the Weapon Being Overlappeed With, and toggles the Widget's visibility
  (`SceneComponent.SetVisibility` (`self.Widget`) false false)
  (set `self.Can Pick ` false))

(event `Print Stats`
  (bind (_max_damage _min_damage) (`self.GetDamageValues`))
  (bind (_max_damage_distance _min_damage_distance) (`self.GetDamage_DistanceValues`))
  (`KismetSystemLibrary.PrintString` (`KismetStringLibrary.Concat_StrStr` (`KismetStringLibrary.Concat_StrStr` "Range" (`KismetStringLibrary.Conv_DoubleToString` (`self.GetRangeValue`))) (`KismetStringLibrary.Concat_StrStr` "Spread" (`KismetStringLibrary.Conv_DoubleToString` (`self.GetSpreadValue`))) (`KismetStringLibrary.Concat_StrStr` "Fire Rate" (`KismetStringLibrary.Conv_DoubleToString` (`self.GetFire_RateValue`))) (`KismetStringLibrary.Concat_StrStr` "Reload Rate" (`KismetStringLibrary.Conv_DoubleToString` (`self.GetReload_RateValue`))) (`KismetStringLibrary.Concat_StrStr` "Controller Recoil" (`KismetStringLibrary.Conv_DoubleToString` (`self.GetController_RecoilValue`))) (`KismetStringLibrary.Concat_StrStr` "Max Damage" (`KismetStringLibrary.Conv_DoubleToString` _max_damage) "Min Damage" (`KismetStringLibrary.Conv_DoubleToString` _min_damage)) (`KismetStringLibrary.Concat_StrStr` "Max Damage Distance" (`KismetStringLibrary.Conv_DoubleToString` _max_damage_distance) "Min Damage Distance" (`KismetStringLibrary.Conv_DoubleToString` _min_damage_distance)))))

(event `Start Spin Weapon`)

(event `End Spin Weapon`)

(fn `NewFunction`)

(fn `Set Weapon Data`
  (bind _returnvalue (`|GetDataTableRow` "/Game/LMS_Game/Characters/Structures/DT_Weapon_Table.DT_Weapon_Table" (`KismetStringLibrary.Conv_StringToName` (`KismetStringLibrary.Conv_IntToString` (`.WeaponID_18_353EC415483F454D94A166BBB6421A63` (break `/Game/LMS_Game/Characters/Structures/S_Weapon_Inventory` (`self.Weapon Inventory `))))))
    (:`then`
      (bind (_weaponname _weapontype _weaponfiretype _weaponammotype _weaponclass _weaponmagsize) (break `/Game/LMS_Game/Characters/Structures/S_Weapon_Struct` _returnvalue))
      (setmembers `/Game/LMS_Game/Characters/Structures/S_Weapon_Struct` :`StructRef` (`self.Weapon_Structure`) :`Weapon Name` _weaponname :`Weapon Type` _weapontype :`Weapon Fire Type` _weaponfiretype :`Weapon Ammo Type` _weaponammotype :`Weapon Class` _weaponclass :`Weapon Mag Size` _weaponmagsize))
    (:`RowNotFound`
      (`KismetSystemLibrary.PrintString` "Data Not Found"))))

(fn `Set Weapon State `
  (params (`Weapon State ` :type "/Game/LMS_Game/Characters/Enums/E_Weapon_State Enum" :default "NewEnumerator0"))
  (bind _weapon_sm (`self.Weapon SM`))
  (bind _weapon_sm_2 (`self.Weapon SM`))
  (bind _weapon_sm_3 (`self.Weapon SM`))
  (bind _weapon_sm_4 (`self.Weapon SM`))
  (switch `/Game/LMS_Game/Characters/Enums/E_Weapon_State` `Weapon State `
    (:`NewEnumerator0`
      ;[0.05098 0.05098 0.05098] Dropped Collision Preset
      (`PrimitiveComponent.SetCollisionProfileName` (`self.Interaction Area`) "OverlapAllDynamic" true)
      (`PrimitiveComponent.SetCollisionProfileName` _weapon_sm_2 "PhysicsActor" true)
      (`PrimitiveComponent.SetCollisionResponseToChannel` _weapon_sm_2 "ECC_Pawn" "ECR_Ignore")
      (`PrimitiveComponent.SetCollisionResponseToChannel` _weapon_sm_2 "ECC_Camera" "ECR_Ignore")
      (`PrimitiveComponent.SetSimulatePhysics` _weapon_sm_2 true))
    (:`NewEnumerator1`
      ;[0.05098 0.05098 0.05098] Equipped Collision Preset
      (`PrimitiveComponent.SetCollisionProfileName` (`self.Interaction Area`) "NoCollision" true)
      (`PrimitiveComponent.SetSimulatePhysics` _weapon_sm_3 false)
      (`PrimitiveComponent.SetCollisionProfileName` _weapon_sm_3 "NoCollision" true)
      (`SceneComponent.K2_AttachToComponent` (`self.Weapon SM`) (`self.DefaultSceneRoot`) "None" "SnapToTarget" "SnapToTarget" "KeepWorld" true))
    (:`NewEnumerator2`
      ;[0.05098 0.05098 0.05098] InHand Collision Preset
      (`PrimitiveComponent.SetCollisionProfileName` (`self.Interaction Area`) "NoCollision" true)
      (`PrimitiveComponent.SetSimulatePhysics` _weapon_sm false)
      (`PrimitiveComponent.SetCollisionProfileName` _weapon_sm "NoCollision" true)
      (`SceneComponent.K2_AttachToComponent` (`self.Weapon SM`) (`self.DefaultSceneRoot`) "None" "SnapToTarget" "SnapToTarget" "KeepWorld" true))
    (:`NewEnumerator3`
      (`PrimitiveComponent.SetCollisionProfileName` (`self.Interaction Area`) "OverlapAllDynamic" true)
      (`PrimitiveComponent.SetCollisionProfileName` _weapon_sm_4 "NoCollision" true)
      (`PrimitiveComponent.SetCollisionResponseToChannel` _weapon_sm_4 "ECC_Pawn" "ECR_Ignore")
      (`PrimitiveComponent.SetCollisionResponseToChannel` _weapon_sm_4 "ECC_Camera" "ECR_Ignore")
      (`PrimitiveComponent.SetSimulatePhysics` _weapon_sm_4 false)
      (`SceneComponent.K2_AttachToComponent` (`self.Weapon SM`) (`self.DefaultSceneRoot`) "None" "SnapToTarget" "SnapToTarget" "KeepWorld" true))))

(fn `UserConstructionScript`
  (bind ((`WeaponMagSize_24_3D837BBD44C9D124D683F1ACF04534E0` _weaponmagsize)) (break `/Game/LMS_Game/Characters/Structures/S_Weapon_Struct` (`self.Weapon_Structure`)))
  (setmembers `/Game/LMS_Game/Characters/Structures/S_Weapon_Inventory` :`StructRef` (`self.Weapon Inventory `) :`Weapon ID` (`.WeaponID_18_353EC415483F454D94A166BBB6421A63` (break `/Game/LMS_Game/Characters/Structures/S_Weapon_Inventory` (`self.Weapon Inventory `))))
  (`self.Set Weapon Data`)
  (setmembers `/Game/LMS_Game/Characters/Structures/S_Weapon_Inventory` :`StructRef` (`self.Weapon Inventory `) :`Current Ammo` (`KismetMathLibrary.RandomIntegerInRange` (/ _weaponmagsize 2) _weaponmagsize)))