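; Gameplay Ability that fires the owner's gun as single, full auto, burst or shotgun, applying GE_IsFiring until it ends.
; Automatic and burst modes loop on a timer until the IsFiring tag is removed or ammo runs out.
; Shots sphere-trace from player camera or AI gun, with aim-reduced spread, recoil and effects.
; Hits apply point damage scaled by distance and bone, then send an IsDamaged gameplay event to the shooter.
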(event `self.K2_ActivateAbility`
  (bind _weapon_ (`self.Get  Owners Gun Ref`))
  (`self.K2_CommitAbility`)
  (`self.BP_ApplyGameplayEffectToOwner` "/Game/LMS_Game/Characters/GAS/Effects/GE_IsFiring.GE_IsFiring_C")
  (`/Engine/EditorBlueprintResources/StandardMacros.IsValid` (`self.Get  Owners Gun Ref`)
    (:`Is Valid`
      (`|ExecutionSequence`
        (:`then_0`
          (`AbilityTask_WaitGameplayTagRemoved.WaitGameplayTagRemove` (struct :`TagName` "Character.Effect.IsFiring") null
            (:`Removed`
              (`self.K2_EndAbility`))))
        (:`then_1`
          (`/Game/LMS_Game/Characters/Weapons/BP_Weapon_Master.Set Weapon Data` _weapon_)
          (switch `/Game/LMS_Game/Characters/Enums/E_Weapon_Fire_Type` (`.WeaponFireType_17_155AF58B4D5E85AF9B0569BD2665F081` (break `/Game/LMS_Game/Characters/Structures/S_Weapon_Struct` (`/Game/LMS_Game/Characters/Weapons/BP_Weapon_Master.Weapon_Structure` _weapon_)))
            (:`NewEnumerator1`
              (set `/Game/LMS_Game/Characters/Character_Logic/BP_LMS_BaseCharacter.Is Firing` true (`self.Get Ability Owner`))
              (`self.Fire Weapon`)
              (`KismetSystemLibrary.Delay` (`LMSWeapon.GetFire_RateValue` (`self.Get  Owners Gun Ref`)))
              (`self.K2_EndAbility`))
            (:`NewEnumerator2`
              (set `/Game/LMS_Game/Characters/Character_Logic/BP_LMS_BaseCharacter.Is Firing` true (`self.Get Ability Owner`))
              (`self.Fire Weapon`)
              (bind _returnvalue (`KismetSystemLibrary.K2_SetTimerDelegate` (`|CreateDelegate` :!event `Fire Weapon`) (`LMSWeapon.GetFire_RateValue` (`self.Get  Owners Gun Ref`)) true))
              (set `self.Full Auto Fire Timer` _returnvalue)
              (`KismetSystemLibrary.Delay` (`LMSWeapon.GetFire_RateValue` (`self.Get  Owners Gun Ref`))))
            (:`NewEnumerator3`
              (set `/Game/LMS_Game/Characters/Character_Logic/BP_LMS_BaseCharacter.Is Firing` true (`self.Get Ability Owner`))
              (`self.Burst Fire`)
              (bind _returnvalue_2 (`KismetSystemLibrary.K2_SetTimerDelegate` (`|CreateDelegate` :!event `Burst Fire`) (`LMSWeapon.GetFire_RateValue` (`self.Get  Owners Gun Ref`)) true))
              (set `self.Full Auto Fire Timer` _returnvalue_2)
              (`KismetSystemLibrary.Delay` (`LMSWeapon.GetFire_RateValue` (`self.Get  Owners Gun Ref`))))
            (:`NewEnumerator4`
              (set `/Game/LMS_Game/Characters/Character_Logic/BP_LMS_BaseCharacter.Is Firing` true (`self.Get Ability Owner`))
              (`self.ShotGun Fire`)
              (`KismetSystemLibrary.Delay` (`LMSWeapon.GetFire_RateValue` (`self.Get  Owners Gun Ref`)))
              (`self.K2_EndAbility`))))))
    (:`Is Not Valid`
      (`self.K2_EndAbility`))))

(event `self.K2_OnEndAbility`
  (params (bWasCancelled :type Boolean))
  (`self.BP_RemoveGameplayEffectFromOwnerWithGrantedTags` (struct :`GameplayTags` (struct :`(TagName` "Character.Effect.IsFiring"))))
  (`KismetSystemLibrary.K2_ClearAndInvalidateTimerHandle` (`self.Full Auto Fire Timer`)))

(event `Fire Weapon`
  (bind _weapon_ (`self.Get  Owners Gun Ref`))
  (bind (_start _end) (`self.Do Trace Math` (`LMSWeapon.GetRangeValue` _weapon_) (`LMSWeapon.GetSpreadValue` _weapon_)))
  (`self.Check For Ammo`
    (:`Ammo Left`
      (bind (_outhit _returnvalue) (`self.Weapon Trace` _start _end))
      (`self.Play Shoot Animation`)
      (`self.Gun Shoot Effects`)
      (`self.Reduce Ammo From Gun`
        (:`Ammo Left`
          (`self.Gun Impact Effetcs` _returnvalue _outhit
            (:`Bullet Hit`
              (`|ExecutionSequence`
                (:`then_1`
                  (`self.Apply Damage Effect` _outhit))))))
        (:`No Ammo Left`
          (`self.K2_EndAbility`))))))

(event `Burst Fire`
  (`self.Fire Weapon`)
  (`KismetSystemLibrary.Delay` 0.1)
  (`self.Fire Weapon`)
  (`KismetSystemLibrary.Delay` 0.1)
  (`self.Fire Weapon`))

(event `ShotGun Fire`
  (bind _weapon_ (`self.Get  Owners Gun Ref`))
  (bind (_start _end) (`self.Do Trace Math` (`LMSWeapon.GetRangeValue` _weapon_) (`LMSWeapon.GetSpreadValue` _weapon_)))
  (`self.Check For Ammo`
    (:`Ammo Left`
      (for _ (range 1 9)
        (bind (_outhit _returnvalue) (`self.Weapon Trace` _start _end))
        (`self.Gun Impact Effetcs` _returnvalue _outhit
          (:`Bullet Hit`
            (`|ExecutionSequence`
              (:`then_1`
                (`self.Apply Damage Effect` _outhit))))))
      (`self.Play Shoot Animation`)
      (`self.Gun Shoot Effects`)
      (`self.Reduce Ammo From Gun`
        (:`No Ammo Left`
          (`self.K2_EndAbility`))))))

(fn `Do Trace Math`
  (params (Range :type "Float (double-precision)") (Spread :type "Float (double-precision)"))
  (returns (Start :type "Vector Structure") (End :type "Vector Structure"))
  (locals (`Aiming?` :type Boolean :default false) (`Weapon Spread` :type "Float (double-precision)") (`Actor Camera` :type "CameraComponent Object Reference") (`Actor Spring Arm` :type "SpringArmComponent Object Reference") (`IS Player Controlled` :type Boolean :default true))
  (bind _owning_actor (`self.Get Ability Owner`))
  (bind _weapon_ (`self.Get  Owners Gun Ref`))
  (bind _weapon_spread (`local.Weapon Spread`))
  (bind _weapon_spread_2 (`local.Weapon Spread`))
  (bind _spread (`local.Spread`))
  (bind _weapon_spread_3 (`local.Weapon Spread`))
  (bind _weapon_spread_4 (`local.Weapon Spread`))
  (bind _actor_camera (`local.Actor Camera`))
  (bind _actor_camera_2 (`local.Actor Camera`))
  (bind _weapon_spread_5 (`local.Weapon Spread`))
  (bind _weapon_spread_6 (`local.Weapon Spread`))
  (`/Engine/EditorBlueprintResources/StandardMacros.IsValid` _owning_actor
    (:`Is Valid`
      (bind _aiming_ (message `/Game/LMS_Game/Characters/Interfaces/IF_WeaponOwner_Interface.IF Is Aiming?` _owning_actor))
      (set `local.Aiming?` _aiming_)
      (bind (_actor _actor_camera_3 _camera_boom) (message `/Game/LMS_Game/Characters/Interfaces/IF_WeaponOwner_Interface.IF Get Actor References` _owning_actor))
      (set `local.Actor Camera` _actor_camera_3)
      (set `local.Actor Spring Arm` _camera_boom)
      (set `local.Weapon Spread` (`KismetMathLibrary.SelectFloat` (* _spread 0.5) _spread (`local.Aiming?`)))
      (return (select `bool` (`local.IS Player Controlled`) :`false` (`Actor.K2_GetActorLocation` (`self.Get  Owners Gun Ref`)) :`true` (+ (`SceneComponent.K2_GetComponentLocation` _actor_camera) (* (`SceneComponent.GetForwardVector` _actor_camera) (`SpringArmComponent.TargetArmLength` (`local.Actor Spring Arm`))))) (select `bool` (`local.IS Player Controlled`) :`false` (+ (`Actor.K2_GetActorLocation` _weapon_) (* (`KismetMathLibrary.GetForwardVector` (`Actor.K2_GetActorRotation` _weapon_)) (`local.Range`)) (`KismetMathLibrary.MakeVector` (`KismetMathLibrary.RandomFloatInRange` (* _weapon_spread_4 -1.0) _weapon_spread_4) (`KismetMathLibrary.RandomFloatInRange` (* _weapon_spread_5 -1.0) _weapon_spread_5) (`KismetMathLibrary.RandomFloatInRange` (* _weapon_spread_3 -1.0) _weapon_spread_3))) :`true` (+ (`SceneComponent.K2_GetComponentLocation` _actor_camera_2) (* (`SceneComponent.GetForwardVector` _actor_camera_2) (`local.Range`)) (`KismetMathLibrary.MakeVector` (`KismetMathLibrary.RandomFloatInRange` (* _weapon_spread_6 -1.0) _weapon_spread_6) (`KismetMathLibrary.RandomFloatInRange` (* _weapon_spread -1.0) _weapon_spread) (`KismetMathLibrary.RandomFloatInRange` (* _weapon_spread_2 -1.0) _weapon_spread_2))))))))

(fn `Get Base Damage`
  (params (Distance :type "Float (double-precision)"))
  (returns (`Damage Result` :type "Float (double-precision)"))
  (locals (`Local Shot Distance` :type "Float (double-precision)") (`Local Damage` :type "Float (double-precision)"))
  (bind (_max_damage_distance _min_damage_distance) (`LMSWeapon.GetDamage_DistanceValues` (`self.Get  Owners Gun Ref`)))
  (bind (_max_damage_distance_2 _min_damage_distance_2) (`LMSWeapon.GetDamage_DistanceValues` (`self.Get  Owners Gun Ref`)))
  (bind (_max_damage _min_damage) (`LMSWeapon.GetDamageValues` (`self.Get  Owners Gun Ref`)))
  (set `local.Local Shot Distance` Distance)
  (if (<= (`local.Local Shot Distance`) _max_damage_distance_2)
    (set `local.Local Damage` (`LMSWeapon.GetDamageValues` (`self.Get  Owners Gun Ref`)))
    (elif (> (`local.Local Shot Distance`) _min_damage_distance_2)
      (set `local.Local Damage` (`.Min_Damage` (`LMSWeapon.GetDamageValues` (`self.Get  Owners Gun Ref`))))
      (else
        (set `local.Local Damage` (- (`LMSWeapon.GetDamageValues` (`self.Get  Owners Gun Ref`)) (* (/ (- (`local.Local Shot Distance`) _max_damage_distance) (- _min_damage_distance _max_damage_distance)) (- _max_damage _min_damage)))))))
  (return (`local.Local Damage`)))

(fn `Get Location Damage Multiplier`
  (params (`Hit Bone Name` :type Name) (`Base Damage` :type "Float (double-precision)"))
  (returns (`Damage Result` :type "Float (double-precision)") (`Critical Hit Result` :type Boolean))
  (locals (`Local Multiplier` :type "Float (double-precision)") (`Is Critical?` :type Boolean))
  (switch `name` `Hit Bone Name`
    (:`Default`
      (set `local.Local Multiplier` 1.0 :!label _label)
      (set `local.Is Critical?` false))
    (:`pelvis`
      (goto _label))
    (:`spine_01`
      (goto _label))
    (:`spine_02`
      (goto _label))
    (:`spine_03`
      (goto _label))
    (:`spine_04`
      (goto _label))
    (:`spine_05`
      (goto _label))
    (:`clavicle_l`
      (set `local.Local Multiplier` 0.8 :!label _label_2)
      (set `local.Is Critical?` false))
    (:`upperarm_l`
      (set `local.Local Multiplier` 0.7 :!label _label_3)
      (set `local.Is Critical?` false))
    (:`lowerarm_l`
      (goto _label_3))
    (:`hand_l`
      (goto _label_3))
    (:`clavicle_r`
      (goto _label_2))
    (:`upperarm_r`
      (goto _label_3))
    (:`lowerarm_r`
      (goto _label_3))
    (:`hand_r`
      (goto _label_3))
    (:`thigh_l`
      (goto _label_2))
    (:`calf_l`
      (goto _label_3))
    (:`foot_l`
      (goto _label_3))
    (:`thigh_r`
      (goto _label_2))
    (:`calf_r`
      (goto _label_3))
    (:`foot_r`
      (goto _label_3))
    (:`neck_01`
      (set `local.Local Multiplier` 2.0 :!label _label_4)
      (set `local.Is Critical?` true))
    (:`neck_02`
      (goto _label_4))
    (:`head`
      (goto _label_4)))
  (return (* (`local.Base Damage`) (`local.Local Multiplier`)) (`local.Is Critical?`)))

(fn `Play Damage Event`
  (params (GameplayEventData :type "GameplayEventData Structure (by ref)"))
  (bind (_eventtag _instigator _target _optionalobject _optionalobject2 _contexthandle _instigatortags _targettags _eventmagnitude) (break `GameplayEventData` GameplayEventData))
  (`/Engine/EditorBlueprintResources/StandardMacros.NegateFloat` _eventmagnitude
    (:`  `
      (bind _returnvalue (`AbilitySystemBlueprintLibrary.AssignTagSetByCallerMagnitude` (`self.MakeOutgoingGameplayEffectSpec` "/Game/LMS_Game/Characters/GAS/Events_Effects/GE_Character_Damaged.GE_Character_Damaged_C" 0.0) _eventtag _eventmagnitude))
      (`AbilitySystemComponent.BP_ApplyGameplayEffectSpecToTarget` (`AbilitySystemBlueprintLibrary.GetAbilitySystemComponent` (`self.GetAvatarActorFromActorInfo`)) _returnvalue (`AbilitySystemBlueprintLibrary.GetAbilitySystemComponent` _target)))))