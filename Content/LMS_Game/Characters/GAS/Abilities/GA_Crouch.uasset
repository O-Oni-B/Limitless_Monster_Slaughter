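; Gameplay Ability that toggles the owning character's crouch.
; It checks the IsCrouching tag count, runs the CrouchUncrouch macro, then applies the matching crouch state effect and ends.
; Uncrouching retries CrouchLineTrace on a short delay until it passes, then stands the character up.
; Cancellation forces an uncrouch but applies GE_IsNotSprinting instead of GE_IsNotCrouching.
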(event `self.K2_ActivateAbility`
  (`self.K2_CommitAbility`)
  (if (not (>= (`AbilitySystemComponent.GetGameplayTagCount` (`AbilitySystemBlueprintLibrary.GetAbilitySystemComponent` (`self.Get Ability Owner`)) (struct :`TagName` "Character.Effect.IsCrouching")) 1))
    (`self.Crouch/Uncrouch` true)
    (`self.BP_ApplyGameplayEffectToOwner` "/Game/LMS_Game/Characters/GAS/Effects/GE_IsCrouching.GE_IsCrouching_C")
    (else
      (`self.Crouch/Uncrouch` false)
      (`self.BP_ApplyGameplayEffectToOwner` "/Game/LMS_Game/Characters/GAS/Effects/GE_IsNotCrouching.GE_IsNotCrouching_C")))
  (`self.K2_EndAbility`))

(event `self.K2_OnEndAbility`
  (params (bWasCancelled :type Boolean))
  (if bWasCancelled
    (`self.BP_ApplyGameplayEffectToOwner` "/Game/LMS_Game/Characters/GAS/Effects/GE_IsNotSprinting.GE_IsNotSprinting_C")
    (set `/Game/LMS_Game/Characters/Character_Logic/BP_LMS_BaseCharacter.Is Crouching` false (`self.Get Ability Owner`))
    (`self.Crouch/Uncrouch` false)))