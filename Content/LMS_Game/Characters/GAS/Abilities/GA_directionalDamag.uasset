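; Gameplay ability that gives a zombie a directional damage reaction, knocking it away from its attacker.
; On activation it stops the AI brain logic, plays a montage and applies a short root motion constant force along the attacker-to-zombie direction.
; The ability ends when the force finishes, the montage is interrupted or no valid brain exists, and ending restarts the AI logic.
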(event `self.K2_ActivateAbility`
  (bind _owning_actor (`self.Get Ability Owner`))
  (bind (_owning_actor_2 _owning_actor_info) (`self.Get Ability Owner`))
  (bind _asbp_lms_zombie_character (cast `/Game/LMS_Game/Characters/Character_Logic/BP_LMS_Zombie_Character` _owning_actor_2))
  (bind _braincomponent (`AIController.BrainComponent` (`AIBlueprintHelperLibrary.GetAIController` _asbp_lms_zombie_character)))
  (`/Engine/EditorBlueprintResources/StandardMacros.IsValid` _braincomponent
    (:`Is Valid`
      (`BrainComponent.StopLogic` _braincomponent "")
      (`|PlayMontage` (`.SkeletalMeshComponent` (break `GameplayAbilityActorInfo` _owning_actor_info))
        (:`then`
          (`AbilityTask_ApplyRootMotionConstantForce.ApplyRootMotionConstantForce` "None" (`KismetMathLibrary.GetForwardVector` (`KismetMathLibrary.FindLookAtRotation` (`Actor.K2_GetActorLocation` (`/Game/LMS_Game/Characters/Character_Logic/BP_LMS_BaseCharacter.Attacker` _owning_actor)) (`Actor.K2_GetActorLocation` _owning_actor))) 700.0 0.2 false null "MaintainLastRootMotionVelocity"
            (:`OnFinish`
              (`self.K2_EndAbility`))))
        (:`OnInterrupted`
          (`self.K2_EndAbility`))))
    (:`Is Not Valid`
      (`self.K2_EndAbility`))))

(event `self.K2_OnEndAbility`
  (params (bWasCancelled :type Boolean))
  (bind _asbp_lms_zombie_character (cast `/Game/LMS_Game/Characters/Character_Logic/BP_LMS_Zombie_Character` (`self.Get Ability Owner`)))
  (bind _braincomponent (`AIController.BrainComponent` (`AIBlueprintHelperLibrary.GetAIController` _asbp_lms_zombie_character)))
  (`/Engine/EditorBlueprintResources/StandardMacros.IsValid` _braincomponent
    (:`Is Valid`
      (`BrainComponent.StartLogic` _braincomponent))))