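; Gameplay Ability that reloads the owner's gun when its magazine is not full.
; Activation applies an IsReloading effect, blocks equipping and plays the gun's reload montage at its reload rate.
; Montage completion or blend-out refills bullets and ends the ability, while interruption ends it without refilling; ending clears the effect and flags.
; Also holds a spread-based trace helper that the reload flow never calls.
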(event `self.K2_ActivateAbility`
  (bind _weapon_ (`self.Get  Owners Gun Ref`))
  (bind _owning_actor (`self.Get Ability Owner`))
  (`self.K2_CommitAbility`)
  (`self.BP_ApplyGameplayEffectToOwner` "/Game/LMS_Game/Characters/GAS/Effects/GE_IsReloading.GE_IsReloading_C")
  (`/Engine/EditorBlueprintResources/StandardMacros.IsValid` (`self.Get  Owners Gun Ref`)
    (:`Is Valid`
      (`self.Check Current Ammo`
        (:`< Mag Size`
          (set `/Game/LMS_Game/Characters/Character_Logic/BP_LMS_BaseCharacter.Is Reloading` true _owning_actor)
          (set `/Game/LMS_Game/Characters/Character_Logic/BP_LMS_BaseCharacter.Can Equip` false _owning_actor)
          (`/Game/LMS_Game/Characters/Weapons/BP_Weapon_Master.Set Weapon Data` (`self.Get  Owners Gun Ref`))
          (`|PlayMontage` (`.SkeletalMeshComponent` (break `GameplayAbilityActorInfo` (`.Owning Actor Info` (`self.Get Ability Owner`)))) (`/Game/LMS_Game/Characters/Weapons/BP_Weapon_Master.Gun Reload Anim Montage` _weapon_) (`LMSWeapon.GetReload_RateValue` _weapon_)
            (:`OnCompleted`
              (`self.Set Bullets and Reload` :!label _label)
              (`self.K2_EndAbility`))
            (:`OnBlendOut`
              (goto _label))
            (:`OnInterrupted`
              (`self.K2_EndAbility`)
              (`KismetSystemLibrary.PrintString` "Reload Interupted"))))
        (:`== Mag size`
          (`self.K2_EndAbility`))))
    (:`Is Not Valid`
      (`self.K2_EndAbility`))))

(event `self.K2_OnEndAbility`
  (params (bWasCancelled :type Boolean))
  (bind _owning_actor (`self.Get Ability Owner`))
  (`self.BP_RemoveGameplayEffectFromOwnerWithGrantedTags` (struct :`GameplayTags` (struct :`(TagName` "Character.Effect.IsReloading"))))
  (set `/Game/LMS_Game/Characters/Character_Logic/BP_LMS_BaseCharacter.Is Reloading` false _owning_actor)
  (set `/Game/LMS_Game/Characters/Character_Logic/BP_LMS_BaseCharacter.Can Equip` true _owning_actor))

(fn `Do Trace Math`
  (params (Range :type "Float (double-precision)") (Spread :type "Float (double-precision)"))
  (returns (Start :type "Vector Structure") (End :type "Vector Structure"))
  (locals (`Aiming?` :type Boolean :default false) (`Weapon Spread` :type "Float (double-precision)") (`Actor Camera` :type "CameraComponent Object Reference") (`IS Player Controlled` :type Boolean :default true))
  (bind _weapon_ (`self.Get  Owners Gun Ref`))
  (bind _owning_actor (`self.Get Ability Owner`))
  (bind _weapon_spread (`local.Weapon Spread`))
  (bind _weapon_spread_2 (`local.Weapon Spread`))
  (bind _spread (`local.Spread`))
  (bind _weapon_spread_3 (`local.Weapon Spread`))
  (bind _weapon_spread_4 (`local.Weapon Spread`))
  (bind _actor_camera (`local.Actor Camera`))
  (bind _weapon_spread_5 (`local.Weapon Spread`))
  (bind _weapon_spread_6 (`local.Weapon Spread`))
  (`/Engine/EditorBlueprintResources/StandardMacros.IsValid` _owning_actor
    (:`Is Valid`
      (bind _aiming_ (message `/Game/LMS_Game/Characters/Interfaces/IF_WeaponOwner_Interface.IF Is Aiming?` _owning_actor))
      (set `local.Aiming?` _aiming_)
      (bind (_actor _actor_camera_2) (message `/Game/LMS_Game/Characters/Interfaces/IF_WeaponOwner_Interface.IF Get Actor References` _owning_actor))
      (set `local.Actor Camera` _actor_camera_2)
      (set `local.Weapon Spread` (`KismetMathLibrary.SelectFloat` (* _spread 0.5) _spread (`local.Aiming?`)))
      (return (select `bool` (`local.IS Player Controlled`) :`false` (`Actor.K2_GetActorLocation` (`self.Get  Owners Gun Ref`)) :`true` (`SceneComponent.K2_GetComponentLocation` (`local.Actor Camera`))) (select `bool` (`local.IS Player Controlled`) :`false` (+ (`Actor.K2_GetActorLocation` _weapon_) (* (`KismetMathLibrary.GetForwardVector` (`Actor.K2_GetActorRotation` _weapon_)) (`local.Range`)) (`KismetMathLibrary.MakeVector` (`KismetMathLibrary.RandomFloatInRange` (* _weapon_spread_4 -1.0) _weapon_spread_4) (`KismetMathLibrary.RandomFloatInRange` (* _weapon_spread_5 -1.0) _weapon_spread_5) (`KismetMathLibrary.RandomFloatInRange` (* _weapon_spread_3 -1.0) _weapon_spread_3))) :`true` (+ (`SceneComponent.K2_GetComponentLocation` _actor_camera) (* (`SceneComponent.GetForwardVector` _actor_camera) (`local.Range`)) (`KismetMathLibrary.MakeVector` (`KismetMathLibrary.RandomFloatInRange` (* _weapon_spread_6 -1.0) _weapon_spread_6) (`KismetMathLibrary.RandomFloatInRange` (* _weapon_spread -1.0) _weapon_spread) (`KismetMathLibrary.RandomFloatInRange` (* _weapon_spread_2 -1.0) _weapon_spread_2))))))))