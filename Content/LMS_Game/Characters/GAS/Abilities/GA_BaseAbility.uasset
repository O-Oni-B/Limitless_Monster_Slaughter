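; Base gameplay ability for LMS characters, providing shared helper functions and leaving its events empty.
; Owner lookup casts the ability's owner to BP_LMS_BaseCharacter, feeding an upward capsule-radius sphere trace for overhead clearance and an in-hand weapon getter.
; The reload helper fills that weapon's magazine whenever reserve ammo of its type is positive, then subtracts the missing rounds from the weapon component's per-type ammo map.
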(event `Apply Root Motion to Direction`)

(fn `Crouch Line Trace`
  (returns (ReturnValue :type Boolean))
  (bind _owning_actor (`self.Get Ability Owner`))
  (bind _returnvalue (`Actor.K2_GetActorLocation` _owning_actor))
  (bind (_outhit _returnvalue_2) (`KismetSystemLibrary.SphereTraceSingle` _returnvalue (+ _returnvalue (* (`KismetMathLibrary.GetUpVector` (`Actor.K2_GetActorRotation` _owning_actor)) 200.0)) (`CapsuleComponent.GetScaledCapsuleRadius` (`Character.CapsuleComponent` _owning_actor)) "TraceTypeQuery1" false (`|MakeArray` (`self.Get Ability Owner`) :!type "Actor Object Reference")))
  (return (not _returnvalue_2)))

(fn `Get  Owners Gun Ref`
  (returns (`Weapon ` :type "/Game/LMS_Game/Characters/Weapons/BP_Weapon_Master Object Reference"))
  (bind _bpc_weapon_system (`/Game/LMS_Game/Characters/Character_Logic/BP_LMS_BaseCharacter.BPC_Weapon_System` (`self.Get Ability Owner`)))
  (`/Engine/EditorBlueprintResources/StandardMacros.IsValid` _bpc_weapon_system
    (:`Is Valid`
      (return (`/Game/LMS_Game/Characters/Actor_Components/BPC_Weapon_System.In Hand Weapon ` _bpc_weapon_system)))))

(fn `Get Ability Owner`
  (returns (`Owning Actor` :type "/Game/LMS_Game/Characters/Character_Logic/BP_LMS_BaseCharacter Object Reference") (`Owning Actor Info` :type "GameplayAbilityActorInfo Structure"))
  (bind _returnvalue (`self.GetActorInfo`))
  (return (cast `/Game/LMS_Game/Characters/Character_Logic/BP_LMS_BaseCharacter` (`.OwnerActor` (break `GameplayAbilityActorInfo` _returnvalue)) :!pure true) _returnvalue))

(fn `Set Bullets and Reload`
  (locals (`Needed Ammo To Reload ` :type Integer))
  (bind _weapon_ (`self.Get  Owners Gun Ref`))
  (bind _weapon__2 (`self.Get  Owners Gun Ref`))
  (bind _weapon__3 (`self.Get  Owners Gun Ref`))
  (bind ((`WeaponAmmoType_21_5AD8EAAD48DD951860D3B58A54FF9DD4` _weaponammotype)) (break `/Game/LMS_Game/Characters/Structures/S_Weapon_Struct` (`/Game/LMS_Game/Characters/Weapons/BP_Weapon_Master.Weapon_Structure` (`self.Get  Owners Gun Ref`))))
  (bind ((`WeaponAmmoType_21_5AD8EAAD48DD951860D3B58A54FF9DD4` _weaponammotype_2)) (break `/Game/LMS_Game/Characters/Structures/S_Weapon_Struct` (`/Game/LMS_Game/Characters/Weapons/BP_Weapon_Master.Weapon_Structure` _weapon__3)))
  (bind ((`WeaponAmmoType_21_5AD8EAAD48DD951860D3B58A54FF9DD4` _weaponammotype_3) (`WeaponMagSize_24_3D837BBD44C9D124D683F1ACF04534E0` _weaponmagsize)) (break `/Game/LMS_Game/Characters/Structures/S_Weapon_Struct` (`/Game/LMS_Game/Characters/Weapons/BP_Weapon_Master.Weapon_Structure` _weapon_)))
  (bind (_actor _actor_camera _camera_boom _weapon_system_component) (message `/Game/LMS_Game/Characters/Interfaces/IF_WeaponOwner_Interface.IF Get Actor References` (`self.Get Ability Owner`)))
  (if (> (`BlueprintMapLibrary.Map_Find` (`/Game/LMS_Game/Characters/Actor_Components/BPC_Weapon_System.Ammo Type / Ttl Ammo` _weapon_system_component) _weaponammotype_3) 0)
    (set `local.Needed Ammo To Reload ` (- _weaponmagsize (`.CurrentAmmo_16_70B92C3E461952DD4AA8428ED417F3D2` (break `/Game/LMS_Game/Characters/Structures/S_Weapon_Inventory` (`/Game/LMS_Game/Characters/Weapons/BP_Weapon_Master.Weapon Inventory ` _weapon_)))))
    (bind (_actor_2 _actor_camera_2 _camera_boom_2 _weapon_system_component_2) (message `/Game/LMS_Game/Characters/Interfaces/IF_WeaponOwner_Interface.IF Get Actor References` (`self.Get Ability Owner`)))
    (bind _value (`BlueprintMapLibrary.Map_Find` (`/Game/LMS_Game/Characters/Actor_Components/BPC_Weapon_System.Ammo Type / Ttl Ammo` _weapon_system_component_2) _weaponammotype))
    (if (<= _value 0)
      (bind (_actor_3 _actor_camera_3 _camera_boom_3 _weapon_system_component_3) (message `/Game/LMS_Game/Characters/Interfaces/IF_WeaponOwner_Interface.IF Get Actor References` (`self.Get Ability Owner`)))
      (setmembers `/Game/LMS_Game/Characters/Structures/S_Weapon_Inventory` :`StructRef` (`/Game/LMS_Game/Characters/Weapons/BP_Weapon_Master.Weapon Inventory ` _weapon__3) :`Current Ammo` (+ (`.CurrentAmmo_16_70B92C3E461952DD4AA8428ED417F3D2` (break `/Game/LMS_Game/Characters/Structures/S_Weapon_Inventory` (`/Game/LMS_Game/Characters/Weapons/BP_Weapon_Master.Weapon Inventory ` _weapon__3))) (`BlueprintMapLibrary.Map_Find` (`/Game/LMS_Game/Characters/Actor_Components/BPC_Weapon_System.Ammo Type / Ttl Ammo` _weapon_system_component_3) _weaponammotype_2)))
      (bind (_actor_4 _actor_camera_4 _camera_boom_4 _weapon_system_component_4) (message `/Game/LMS_Game/Characters/Interfaces/IF_WeaponOwner_Interface.IF Get Actor References` (`self.Get Ability Owner`)))
      (`BlueprintMapLibrary.Map_Add` (`/Game/LMS_Game/Characters/Actor_Components/BPC_Weapon_System.Ammo Type / Ttl Ammo` _weapon_system_component_4) _weaponammotype_2)
      (else
        (setmembers `/Game/LMS_Game/Characters/Structures/S_Weapon_Inventory` :`StructRef` (`/Game/LMS_Game/Characters/Weapons/BP_Weapon_Master.Weapon Inventory ` _weapon__2) :`Current Ammo` (`.WeaponMagSize_24_3D837BBD44C9D124D683F1ACF04534E0` (break `/Game/LMS_Game/Characters/Structures/S_Weapon_Struct` (`/Game/LMS_Game/Characters/Weapons/BP_Weapon_Master.Weapon_Structure` _weapon__2))))
        (bind (_actor_5 _actor_camera_5 _camera_boom_5 _weapon_system_component_5) (message `/Game/LMS_Game/Characters/Interfaces/IF_WeaponOwner_Interface.IF Get Actor References` (`self.Get Ability Owner`)))
        (`BlueprintMapLibrary.Map_Add` (`/Game/LMS_Game/Characters/Actor_Components/BPC_Weapon_System.Ammo Type / Ttl Ammo` _weapon_system_component_5) _weaponammotype (- _value (`local.Needed Ammo To Reload `)))))))