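; Gameplay Ability that puts the owning actor into an aiming state.
; On activation it commits, then, if the actor is not already aiming, calls its start-aim hook and applies the GE_IsAiming effect.
; It waits for the IsAiming tag to be removed to end itself, then calls the end-aim hook.
; Removal of the effect is left to outside logic, as the ability's own removal node is unwired.
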(event `self.K2_ActivateAbility`
  (`self.K2_CommitAbility`)
  (if (not (`/Game/LMS_Game/Characters/Character_Logic/BP_LMS_BaseCharacter.Is Aiming` (`self.Get Ability Owner`)))
    (`/Game/LMS_Game/Characters/Character_Logic/BP_LMS_BaseCharacter.On Start Aim` (`self.Get Ability Owner`))
    (`self.BP_ApplyGameplayEffectToOwner` "/Game/LMS_Game/Characters/GAS/Effects/GE_IsAiming.GE_IsAiming_C"))
  (bind _asynctaskproxy (`AbilityTask_WaitGameplayTagRemoved.WaitGameplayTagRemove` (struct :`TagName` "Character.Effect.IsAiming") null)
    (:`then`
      (set `self.Aim Async Task` _asynctaskproxy))
    (:`Removed`
      (`self.K2_EndAbility`))))

(event `self.K2_OnEndAbility`
  (params (bWasCancelled :type Boolean))
  (`/Game/LMS_Game/Characters/Character_Logic/BP_LMS_BaseCharacter.On End Aim` (`self.Get Ability Owner`)))