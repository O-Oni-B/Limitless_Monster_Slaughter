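; GA_Sprint is a Gameplay Ability that toggles sprinting on the owning character each time it activates.
; It flips the actor's IsSprinting flag, sets CharacterMovement MaxWalkSpeed through a helper, and applies GE_IsSprinting or GE_IsNotSprinting to the owner.
; The ability ends immediately after each toggle.
; If cancelled, OnEndAbility restores walking speed, applies the not-sprinting effect and clears the flag.
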(event `self.K2_ActivateAbility`
  (`self.K2_CommitAbility`)
  (if (not (`/Game/LMS_Game/Characters/Character_Logic/BP_LMS_BaseCharacter.Is Sprinting` (`self.Get Ability Owner`)))
    (set `/Game/LMS_Game/Characters/Character_Logic/BP_LMS_BaseCharacter.Is Sprinting` true (`self.Get Ability Owner`))
    (`self.Set Walk Speed` 600.0)
    (`self.BP_ApplyGameplayEffectToOwner` "/Game/LMS_Game/Characters/GAS/Effects/GE_IsSprinting.GE_IsSprinting_C")
    (else
      (set `/Game/LMS_Game/Characters/Character_Logic/BP_LMS_BaseCharacter.Is Sprinting` false (`self.Get Ability Owner`))
      (`self.Set Walk Speed` 300.0)
      (`self.BP_ApplyGameplayEffectToOwner` "/Game/LMS_Game/Characters/GAS/Effects/GE_IsNotSprinting.GE_IsNotSprinting_C")))
  (`self.K2_EndAbility`))

(event `self.K2_OnEndAbility`
  (params (bWasCancelled :type Boolean))
  (if bWasCancelled
    (`self.Set Walk Speed` 300.0)
    (`self.BP_ApplyGameplayEffectToOwner` "/Game/LMS_Game/Characters/GAS/Effects/GE_IsNotSprinting.GE_IsNotSprinting_C")
    (set `/Game/LMS_Game/Characters/Character_Logic/BP_LMS_BaseCharacter.Is Sprinting` false (`self.Get Ability Owner`))))