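; Zombie enemy character for the LMS game mode, counted in EnemiesAlive, with a randomized walk speed.
; Attacks play a random montage and enable hand and mouth overlaps, which deal point damage to other teams through a once-only gate reset shortly after overlap ends.
; Death ragdolls the mesh, adding a hit impulse for non-explosion kills, then notifies the game mode, spawns random pickups and destroys the actor after a delay.
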(event `self.ReceiveBeginPlay`
  (`parent.ReceiveBeginPlay`)
  (bind _asbp_lms_game_mode (cast `/Game/LMS_Game/Characters/Character_Logic/BP_LMS_GameMode` (`GameplayStatics.GetGameMode`)))
  (`/Engine/EditorBlueprintResources/StandardMacros.IncrementInt` (`/Game/LMS_Game/Characters/Character_Logic/BP_LMS_GameMode.Enemies Alive` _asbp_lms_game_mode)))

(event `Stop Attack`)

(event `Attack`
  (bind _zombie_attack_montages (`self.Zombie Attack Montages`))
  (`self.Setting Hand Collision Enabled`)
  (set `self.Attack Index` (`.OutIndex` (`KismetArrayLibrary.Array_Random` _zombie_attack_montages)))
  (`|PlayMontage` (`self.Mesh`) (`|GetArrayItem` _zombie_attack_montages (`self.Attack Index`))
    (:`OnCompleted`
      _)
    (:`OnBlendOut`
      _)
    (:`OnInterrupted`
      _))
  (`self.On Attack End`)
  (`PrimitiveComponent.SetCollisionEnabled` (`self.Hand_r`) "NoCollision")
  (`PrimitiveComponent.SetCollisionEnabled` (`self.Hand_l`) "NoCollision"))

(event `self.Hand_l.OnComponentBeginOverlap`
  (params (OverlappedComponent :type "PrimitiveComponent Object Reference") (OtherActor :type "Actor Object Reference") (OtherComp :type "PrimitiveComponent Object Reference") (OtherBodyIndex :type Integer) (bFromSweep :type Boolean) (SweepResult :type "HitResult Structure (by ref)"))
  (`self.Deal Damage` SweepResult (`self.Hand_l`) 3.5 :!label _label))

(event `self.Hand_r.OnComponentEndOverlap`
  (params (OverlappedComponent :type "PrimitiveComponent Object Reference") (OtherActor :type "Actor Object Reference") (OtherComp :type "PrimitiveComponent Object Reference") (OtherBodyIndex :type Integer))
  (`KismetSystemLibrary.Delay` 0.5)
  (`self.Reset Damage`))

(event `Reset Damage`
  (`|ExecutionSequence`
    (:`then_0`
      (goto _label :!via `Reset`))
    (:`then_1`
      (goto _label_2 :!via `Reset`))
    (:`then_2`
      (goto _label_3 :!via `Reset`))))

(event `self.Hand_l.OnComponentEndOverlap`
  (params (OverlappedComponent :type "PrimitiveComponent Object Reference") (OtherActor :type "Actor Object Reference") (OtherComp :type "PrimitiveComponent Object Reference") (OtherBodyIndex :type Integer))
  (`KismetSystemLibrary.Delay` 0.5)
  (`self.Reset Damage`))

(event `self.Hand_r.OnComponentBeginOverlap`
  (params (OverlappedComponent :type "PrimitiveComponent Object Reference") (OtherActor :type "Actor Object Reference") (OtherComp :type "PrimitiveComponent Object Reference") (OtherBodyIndex :type Integer) (bFromSweep :type Boolean) (SweepResult :type "HitResult Structure (by ref)"))
  (`self.Deal Damage` SweepResult (`self.Hand_r`) 3.5 :!label _label_2))

(event `self.Mouth.OnComponentEndOverlap`
  (params (OverlappedComponent :type "PrimitiveComponent Object Reference") (OtherActor :type "Actor Object Reference") (OtherComp :type "PrimitiveComponent Object Reference") (OtherBodyIndex :type Integer))
  (`KismetSystemLibrary.Delay` 0.5)
  (`self.Reset Damage`))

(event `self.Mouth.OnComponentBeginOverlap`
  (params (OverlappedComponent :type "PrimitiveComponent Object Reference") (OtherActor :type "Actor Object Reference") (OtherComp :type "PrimitiveComponent Object Reference") (OtherBodyIndex :type Integer) (bFromSweep :type Boolean) (SweepResult :type "HitResult Structure (by ref)"))
  (`self.Deal Damage` SweepResult (`self.Mouth`) 6.0 :!label _label_3))

(event `self.Death`
  (params (`Death Causer` :type "Actor Object Reference") (`Hit ` :type "HitResult Structure") (`Explosion Damage?` :type Boolean))
  (bind _returnvalue (`KismetMathLibrary.RandomInteger` 6))
  (`self.Checking And Playing Character Death ` `Hit ` `Explosion Damage?`)
  (`/Engine/EditorBlueprintResources/StandardMacros.DoOnce` false
    (:`Completed`
      (bind _asbp_lms_game_mode (cast `/Game/LMS_Game/Characters/Character_Logic/BP_LMS_GameMode` (`GameplayStatics.GetGameMode`))
        (:`then`
          (`/Engine/EditorBlueprintResources/StandardMacros.DecrementInt` (`/Game/LMS_Game/Characters/Character_Logic/BP_LMS_GameMode.Enemies Alive` _asbp_lms_game_mode)
            (:`  `
              (`/Game/LMS_Game/Characters/Character_Logic/BP_LMS_GameMode.Check Enemy Left` _asbp_lms_game_mode)
              (`/Game/LMS_Game/Characters/Character_Logic/BP_LMS_GameMode.Event Dead Enemy` _asbp_lms_game_mode))))
        (:`CastFailed`
          _))
      (for _ (range (+ _returnvalue 1))
        (`|SpawnActorFromClass` (select `int` _returnvalue :`0` "/Game/LMS_Game/Characters/Weapons/PickUps/BP_HeavyAmmo_PickUp.BP_HeavyAmmo_PickUp_C" :`1` "/Game/LMS_Game/Characters/Weapons/PickUps/BP_LightAmmo_PickUp.BP_LightAmmo_PickUp_C" :`2` "/Game/LMS_Game/Characters/Weapons/PickUps/BP_MediumAmmo_PickUp.BP_MediumAmmo_PickUp_C" :`3` "/Game/LMS_Game/Characters/Weapons/PickUps/BP_ShotGunAmmo_PickUp.BP_ShotGunAmmo_PickUp_C" :`4` "/Game/LMS_Game/Characters/Weapons/PickUps/BP_Grenade_PickUp.BP_Grenade_PickUp_C" :`5` "/Game/LMS_Game/Characters/Weapons/PickUps/BP_Drink_PickUp.BP_Drink_PickUp_C" :!type "Actor Class Reference") (`self.GetTransform`) "AlwaysSpawn" "OverrideRootScale" null null))
      (`KismetSystemLibrary.K2_SetTimerDelegate` (delegate `Destroy Actor`) 5.0))))

(event `Destroy Actor`
  (`self.K2_DestroyActor`))

(fn `Get Character Team`
  (returns (Teams :type "/Game/LMS_Game/Characters/Enums/E_AI_Teams Enum"))
  (return "NewEnumerator2"))

(fn `IF Get Actor References`
  (returns (Actor :type "Character Object Reference") (`Actor Camera` :type "CameraComponent Object Reference") (`Camera Boom` :type "SpringArmComponent Object Reference") (`Weapon System Component` :type "/Game/LMS_Game/Characters/Actor_Components/BPC_Weapon_System Object Reference") (`Damage System Component ` :type "/Game/LMS_Game/Characters/Actor_Components/BPC_Damage_System Object Reference"))
  (return self null null null null))

(fn `IF Get Equipped Weapon Input `
  (returns (`Weapon Input` :type "/Game/LMS_Game/Characters/Enums/E_Weapon_Inputs Enum"))
  (bind _bpc_weapon_system (`self.BPC_Weapon_System`))
  (`/Engine/EditorBlueprintResources/StandardMacros.IsValid` _bpc_weapon_system
    (:`Is Valid`
      (return (`/Game/LMS_Game/Characters/Actor_Components/BPC_Weapon_System.Weapon Input ` _bpc_weapon_system)))))

(fn `IF Is Dead`
  (returns (`Dead?` :type Boolean))
  (return (`self.Dead?`)))

(fn `Set Enemy Speed`
  (params (Speed :type "/Game/LMS_Game/Characters/Enums/E_MovementSpeed Enum" :default "NewEnumerator0"))
  (returns (`Speed Value` :type "Float (double-precision)"))
  (bind _output_get (set `CharacterMovementComponent.MaxWalkSpeed` (select `/Game/LMS_Game/Characters/Enums/E_MovementSpeed` Speed :`NewEnumerator1` 10.0 :`NewEnumerator2` 200.0 :`NewEnumerator3` 500.0 :!type "Float (single-precision)") (`self.CharacterMovement`)))
  (return _output_get))

(fn `Set State Attacking`
  (params (`Atacking State` :type Boolean))
  (returns (`Attacking State?` :type Boolean))
  (bind _output_get (set `self.Atacking State` `Atacking State`))
  (return _output_get))

(fn `UserConstructionScript`
  (`parent.UserConstructionScript`)
  (set `CharacterMovementComponent.MaxWalkSpeed` (`KismetMathLibrary.RandomFloatInRange` 50.0 500.0) (`self.CharacterMovement`)))