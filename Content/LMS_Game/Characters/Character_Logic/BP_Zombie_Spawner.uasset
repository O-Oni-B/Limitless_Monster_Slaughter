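; BP_Zombie_Spawner is a placeable actor that spawns BP_LMS_Zombie_Character enemies around its own location.
; BeginPlay starts a looping timer, after a short initial delay, that fires a spawn event.
; Each spawn picks a random reachable navmesh point within a radius of the spawner and increments a counter.
; Once the counter hits its limit of ten, the timer is cleared, so spawning stops.
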(event `self.ReceiveBeginPlay`
  (bind _returnvalue (`KismetSystemLibrary.K2_SetTimerDelegate` (delegate `Spawn Enemy`) 1.0 true 5.0))
  (set `self.Spawner Timer` _returnvalue))

(event `Spawn Enemy`
  (`|SpawnActorFromClass` "/Game/LMS_Game/Characters/Character_Logic/BP_LMS_Zombie_Character.BP_LMS_Zombie_Character_C" (`KismetMathLibrary.MakeTransform` (`NavigationSystemV1.K2_GetRandomReachablePointInRadius` (`self.K2_GetActorLocation`) 500.0 null null)) "Undefined" "OverrideRootScale" null null)
  (bind _result (`/Engine/EditorBlueprintResources/StandardMacros.IncrementInt` (`self.Zombie Count`))
    (:`  `
      (set `self.Zombie Count` _result)
      (if (>= (`self.Zombie Count`) 10)
        (`KismetSystemLibrary.K2_ClearAndInvalidateTimerHandle` (`self.Spawner Timer`))))))

(fn `UserConstructionScript`)