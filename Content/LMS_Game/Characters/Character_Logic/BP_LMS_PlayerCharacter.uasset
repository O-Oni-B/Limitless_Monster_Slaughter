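; Player character Blueprint for LMS, handling the HUD, cameras, damage and death.
; Shift+C toggles the two cameras, while timelines smooth boom length, offset and FOV for crouching and aiming.
; Point damage applies a gameplay effect, blood and camera shake, dropping weapons at zero health.
; Death ragdolls the body, with a directional impulse for non-explosion kills, shows game over and spawns pickups from the weapon component's ammo and items.
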(event `self.ReceiveBeginPlay`
  (`|ExecutionSequence`
    (:`then_1`
      (`parent.ReceiveBeginPlay`)
      (bind _returnvalue (`|CreateWidget` "/Game/LMS_Game/UI/Player_HUD.Player_HUD_C" (`GameplayStatics.GetPlayerController` 0)))
      (set `self.HUD_Ref` _returnvalue)
      (`UserWidget.AddToViewport` _returnvalue 0))))

(event `Key|Shift+C`
  (params (Key :type "Key Structure"))
  (:`Pressed`
    (if (`self.FPP Camera?`)
      (`/Engine/EditorBlueprintResources/StandardMacros.FlipFlop`
        (:`A`
          (set `self.TPP Camera?` true)
          (`ActorComponent.SetActive` (`self.TTP_Camera`) true false)
          (`ActorComponent.SetActive` (`self.FTP_Camera`) false false))
        (:`B`
          (set `self.FPP Camera?` true)
          (`ActorComponent.SetActive` (`self.TTP_Camera`) false false)
          (`ActorComponent.SetActive` (`self.FTP_Camera`) true false))))))

(event `self.K2_OnStartCrouch`
  (params (HalfHeightAdjust :type "Float (single-precision)") (ScaledHalfHeightAdjust :type "Float (single-precision)"))
  (`self.Attaching Camera Component` (`self.TTP_CameraBoom`) (`self.TTP_Camera`) (`self.Mesh`) "spine_01"
    (:`Completed`
      (bind (_direction _crouch_alpha) (`Timeline|Crouch Camera Smoothing` :!label _label)
        (:`Update`
          (if (not (`self.Is Aiming`))
            (set `SpringArmComponent.TargetArmLength` (`KismetMathLibrary.Lerp` 300.0 450.0 _crouch_alpha) (`self.TTP_CameraBoom`))))))))

(event `self.K2_OnEndCrouch`
  (params (HalfHeightAdjust :type "Float (single-precision)") (ScaledHalfHeightAdjust :type "Float (single-precision)"))
  (`self.Attaching Camera Component` (`self.TTP_CameraBoom`) (`self.TTP_Camera`) (`self.CapsuleComponent`)
    (:`Completed`
      (goto _label :!via `Reverse`))))

(event `self.Start Aim`
  (bind _ttp_cameraboom (`self.TTP_CameraBoom`))
  (set `self.Is Aiming` true)
  (set `SpringArmComponent.bEnableCameraLag` false _ttp_cameraboom)
  (set `SpringArmComponent.bEnableCameraRotationLag` false _ttp_cameraboom)
  (bind (_direction _aim_track) (`Timeline|Aim Smoothing` :!label _label_2)
    (:`Update`
      (if (`NavMovementComponent.IsCrouching` (`self.CharacterMovement`))
        (set `SpringArmComponent.TargetArmLength` (`KismetMathLibrary.Lerp` 450.0 100.0 _aim_track) (`self.TTP_CameraBoom`))
        (set `SpringArmComponent.SocketOffset` (`KismetMathLibrary.VLerp` (0.0 50.0 60.0) (0.0 65.0 70.0) _aim_track) (`self.TTP_CameraBoom`))
        (`CameraComponent.SetFieldOfView` (`self.TTP_Camera`) (`KismetMathLibrary.Lerp` 90.0 70.0 _aim_track))
        (else
          (set `SpringArmComponent.TargetArmLength` (`KismetMathLibrary.Lerp` 300.0 100.0 _aim_track) (`self.TTP_CameraBoom`))
          (set `SpringArmComponent.SocketOffset` (`KismetMathLibrary.VLerp` (0.0 50.0 60.0) (0.0 65.0 70.0) _aim_track) (`self.TTP_CameraBoom`))
          (`CameraComponent.SetFieldOfView` (`self.TTP_Camera`) (`KismetMathLibrary.Lerp` 90.0 70.0 _aim_track)))))))

(event `self.End Aim`
  (bind _ttp_cameraboom (`self.TTP_CameraBoom`))
  (set `self.Is Aiming` false)
  (set `SpringArmComponent.bEnableCameraLag` true _ttp_cameraboom)
  (set `SpringArmComponent.bEnableCameraRotationLag` true _ttp_cameraboom)
  (goto _label_2 :!via `Reverse`))

(event `self.ReceivePointDamage`
  (params (Damage :type "Float (single-precision)") (DamageType :type "DamageType Object Reference") (HitLocation :type "Vector Structure") (HitNormal :type "Vector Structure") (HitComponent :type "PrimitiveComponent Object Reference") (BoneName :type Name) (ShotFromDirection :type "Vector Structure") (InstigatedBy :type "Controller Object Reference") (DamageCauser :type "Actor Object Reference") (HitInfo :type "HitResult Structure (by ref)"))
  (add `self.On Death` (`|CreateDelegate` :!event `Death`))
  (bind _result (`self.Apply Damage Function` Damage (struct :`TagName` "Character.Event.IsDamaged") "/Game/LMS_Game/Characters/GAS/Events_Effects/GE_Character_Damaged.GE_Character_Damaged_C"))
  (`|ExecutionSequence`
    (:`then_0`
      (if (<= (`self.GetHealthValues`) 0.0)
        (`self.Drop All Weapons`
          (:`Continue`
            (`self.On Death` DamageCauser HitInfo)))))
    (:`then_1`
      (`self.Apply Damage` HitInfo)
      (`AISense_Damage.ReportDamageEvent` self DamageCauser _result HitLocation))))

(event `self.Death`
  (params (`Death Causer` :type "Actor Object Reference") (`Hit ` :type "HitResult Structure") (`Explosion Damage?` :type Boolean))
  (bind _returnvalue (`self.GetTransform`))
  (bind _returnvalue_2 (`GameplayStatics.GetPlayerController` 0))
  (bind _bpc_weapon_system (`self.BPC_Weapon_System`))
  (bind _item_inventory (`/Game/LMS_Game/Characters/Actor_Components/BPC_Weapon_System.Item Inventory` _bpc_weapon_system))
  (`self.Checking And Playing Character Death ` `Hit ` `Explosion Damage?`)
  (`Widget.RemoveFromParent` (`self.HUD_Ref`))
  (bind _returnvalue_3 (`|CreateWidget` "/Game/LMS_Game/UI/WB_GameOverMenu.WB_GameOverMenu_C"))
  (`UserWidget.AddToViewport` _returnvalue_3 0)
  (set `PlayerController.bShowMouseCursor` true _returnvalue_2)
  (`WidgetBlueprintLibrary.SetInputMode_UIOnlyEx` _returnvalue_2 null)
  (bind _keys (`BlueprintMapLibrary.Map_Keys` (`/Game/LMS_Game/Characters/Actor_Components/BPC_Weapon_System.Ammo Type / Ttl Ammo` _bpc_weapon_system)))
  (for _array_element _keys
    (switch `/Game/LMS_Game/Characters/Enums/E_Ammo_Type` _array_element
      (:`NewEnumerator1`
        (bind _value (`BlueprintMapLibrary.Map_Find` (`/Game/LMS_Game/Characters/Actor_Components/BPC_Weapon_System.Ammo Type / Ttl Ammo` (`self.BPC_Weapon_System`)) _array_element))
        (`|SpawnActorFromClass` "/Game/LMS_Game/Characters/Weapons/PickUps/BP_HeavyAmmo_PickUp.BP_HeavyAmmo_PickUp_C" _returnvalue "Undefined" "OverrideRootScale" null _value null))
      (:`NewEnumerator2`
        (`|SpawnActorFromClass` "/Game/LMS_Game/Characters/Weapons/PickUps/BP_MediumAmmo_PickUp.BP_MediumAmmo_PickUp_C" _returnvalue "Undefined" "OverrideRootScale" null _value null))
      (:`NewEnumerator3`
        (`|SpawnActorFromClass` "/Game/LMS_Game/Characters/Weapons/PickUps/BP_LightAmmo_PickUp.BP_LightAmmo_PickUp_C" _returnvalue "Undefined" "OverrideRootScale" null _value null))
      (:`NewEnumerator4`
        (`|SpawnActorFromClass` "/Game/LMS_Game/Characters/Weapons/PickUps/BP_ShotGunAmmo_PickUp.BP_ShotGunAmmo_PickUp_C" _returnvalue "Undefined" "OverrideRootScale" null _value null))))
  (bind _keys_2 (`BlueprintMapLibrary.Map_Keys` _item_inventory))
  (for _array_element_2 _keys_2
    (switch `/Game/LMS_Game/Characters/Enums/E_Item_Type` _array_element_2
      (:`NewEnumerator0`
        (bind _value_2 (`BlueprintMapLibrary.Map_Find` _item_inventory _array_element_2))
        (`|SpawnActorFromClass` "/Game/LMS_Game/Characters/Weapons/PickUps/BP_Grenade_PickUp.BP_Grenade_PickUp_C" _returnvalue "Undefined" "OverrideRootScale" null _value_2 null))
      (:`NewEnumerator1`
        (`|SpawnActorFromClass` "/Game/LMS_Game/Characters/Weapons/PickUps/BP_Drink_PickUp.BP_Drink_PickUp_C" _returnvalue "Undefined" "OverrideRootScale" null _value_2 null)))))

(fn `IF Get Actor References`
  (returns (Actor :type "Character Object Reference") (`Actor Camera` :type "CameraComponent Object Reference") (`Camera Boom` :type "SpringArmComponent Object Reference") (`Weapon System Component` :type "/Game/LMS_Game/Characters/Actor_Components/BPC_Weapon_System Object Reference") (`Damage System Component ` :type "/Game/LMS_Game/Characters/Actor_Components/BPC_Damage_System Object Reference"))
  (return self (`self.TTP_Camera`) (`self.TTP_CameraBoom`) (`self.BPC_Weapon_System`) null))

(fn `IF Get Equipped Weapon Input `
  (returns (`Weapon Input` :type "/Game/LMS_Game/Characters/Enums/E_Weapon_Inputs Enum"))
  (bind _bpc_weapon_system (`self.BPC_Weapon_System`))
  (`/Engine/EditorBlueprintResources/StandardMacros.IsValid` _bpc_weapon_system
    (:`Is Valid`
      (return (`/Game/LMS_Game/Characters/Actor_Components/BPC_Weapon_System.Weapon Input ` _bpc_weapon_system)))))

(fn `UserConstructionScript`
  (`parent.UserConstructionScript`))