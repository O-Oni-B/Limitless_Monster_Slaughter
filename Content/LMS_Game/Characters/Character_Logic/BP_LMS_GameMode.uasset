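; BP_LMS_GameMode is the game mode that tracks zombie waves and the count of living enemies.
; CheckEnemyLeft calls SpawnNextWave and then increments ZombieWave once EnemiesAlive reaches zero; the count is not changed in this graph.
; HitEnemy and DeadEnemy events forward to matching Call functions, while the DeleteUnusedPickUps call is unconnected.
; Tick prints the enemy count and wave number on screen every frame as debug text.
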(event `Check Enemy Left`
  (if (== (`self.Enemies Alive`) 0)
    (`self.Spawn Next Wave`)
    (`/Engine/EditorBlueprintResources/StandardMacros.IncrementInt` (`self.Zombie Wave`))))

(event `self.ReceiveTick`
  (params (DeltaSeconds :type "Float (single-precision)"))
  (`KismetSystemLibrary.PrintString` (`KismetStringLibrary.Concat_StrStr` "Total Enemies Alive: " (`KismetStringLibrary.Conv_IntToString` (`self.Enemies Alive`))) true true (struct :`R` 1.0 :`B` 0.592294 :`A` 1.0) 0.0)
  (`KismetSystemLibrary.PrintString` (`KismetStringLibrary.Concat_StrStr` "Wave Number: " (`KismetStringLibrary.Conv_IntToString` (`self.Zombie Wave`))) true true (struct :`R` 1.0 :`B` 0.592294 :`A` 1.0) 0.0))

(event `Event Hit Enemy`
  (`self.Hit Enemy`))

(event `Event Dead Enemy`
  (`self.Dead Enemy`))

(fn `UserConstructionScript`)