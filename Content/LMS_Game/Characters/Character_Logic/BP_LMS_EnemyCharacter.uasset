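; Enemy character Blueprint for the LMS game, extending a parent character class with weapon-system, team and state accessors.
; BeginPlay starts a full-reload async actor load with debug prints for the result, then runs the parent's BeginPlay.
; Interface-style functions expose the weapon component and its input, death state, a fixed team and attacking state.
; A helper snaps a component to a socket, and an unconnected shotgun spawn remains in the graph.
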(event `self.ReceiveBeginPlay`
  (`|ExecutionSequence`
    (:`then_0`
      (`EMSAsyncLoadGame.AsyncLoadActors` 1 true
        (:`OnCompleted`
          (`KismetSystemLibrary.PrintString` "Loaded Succesfully"))
        (:`OnFailed`
          (`KismetSystemLibrary.PrintString` "Loaded Failed"))))
    (:`then_1`
      (`parent.ReceiveBeginPlay`))))

(fn `Get Character Team`
  (returns (Teams :type "/Game/LMS_Game/Characters/Enums/E_AI_Teams Enum"))
  (return "NewEnumerator0"))

(fn `IF Get Actor References`
  (returns (Actor :type "Character Object Reference") (`Actor Camera` :type "CameraComponent Object Reference") (`Camera Boom` :type "SpringArmComponent Object Reference") (`Weapon System Component` :type "/Game/LMS_Game/Characters/Actor_Components/BPC_Weapon_System Object Reference") (`Damage System Component ` :type "/Game/LMS_Game/Characters/Actor_Components/BPC_Damage_System Object Reference"))
  (return self null null (`self.BPC_Weapon_System`) null))

(fn `IF Get Equipped Weapon Input `
  (returns (`Weapon Input` :type "/Game/LMS_Game/Characters/Enums/E_Weapon_Inputs Enum"))
  (bind _bpc_weapon_system (`self.BPC_Weapon_System`))
  (`/Engine/EditorBlueprintResources/StandardMacros.IsValid` _bpc_weapon_system
    (:`Is Valid`
      (return (`/Game/LMS_Game/Characters/Actor_Components/BPC_Weapon_System.Weapon Input ` _bpc_weapon_system)))))

(fn `IF Is Dead`
  (returns (`Dead?` :type Boolean))
  (return (`self.Dead?`)))

(fn `Set State Attacking`
  (params (`Atacking State` :type Boolean))
  (returns (`Attacking State?` :type Boolean))
  (bind _output_get (set `self.Atacking State` `Atacking State`))
  (return _output_get))

(fn `UserConstructionScript`
  (`parent.UserConstructionScript`))