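; Actor component for any Character that manages weapon pickup, holstering, equipping, swapping and dropping across two rifle, one handgun and one melee slot.
; Pickup picks a holster by weapon type, recursively retrying after freeing space when full.
; Slot inputs trigger the GA_EquipWeapon ability or EquipEvent directly, which reattaches weapons between hand and holster sockets.
; It also switches combat/non-combat movement settings and holds mostly stubbed interface getters.
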(event `self.ReceiveBeginPlay`
  ;[0.05098 0.05098 0.05098] Getting Owner Ref - Casting to Character class since this actor component can be attached to any Character Blueprint
  (bind _ascharacter (cast `Character` (`self.GetOwner`)))
  (bind _output_get (set `self.Character Ref ` _ascharacter))
  (set `self.Character Movement` (`Character.CharacterMovement` _output_get)))

(event `Equip Event`
  (bind _weapon_input_ (`self.Weapon Input `))
  (bind _weapon_ (`self.Get Weapons Based on Inputs` _weapon_input_))
  ;[0.05098 0.05098 0.05098] Equip Event - This function does a bunch of checks with the Weapon Input Enum, and equips or swaps the weapons depending on those conditions
  (if (`|EnumInequality` (`self.Weapon Input `) "NewEnumerator0")
    (if (`self.Has Weapon Equiped?`)
      (if (`|EnumInequality` _weapon_input_ "NewEnumerator4")
        (`self.Swap Weapon` _weapon_)
        (else
          (`self.Equip/Unequip` _weapon_)
          (set `self.Rifle Equipped?` false)
          (set `self.Hand Gun Equipped?` false)
          (set `self.Mellee Equipped?` false)))
      (elif (`|EnumInequality` (`self.Weapon Input `) "NewEnumerator4")
        (`self.Equip/Unequip` (`self.Get Weapons Based on Inputs` (`self.Weapon Input `)) true)))))

(event `Equip Weapon`
  (params (`Weapon Input ` :type "/Game/LMS_Game/Characters/Enums/E_Weapon_Inputs Enum" :default "NewEnumerator0"))
  (`self.Checking Equiping Conditions` (`self.Get Weapons Based on Inputs` `Weapon Input `)
    (:`Can Switch`
      (`self.Equiping A Weapon Based on Input` `Weapon Input `))
    (:`Sheeth`
      (`self.Equiping A Weapon Based on Input` "NewEnumerator4"))))

(event `Drop Weapon`
  (params (`Weapon to Drop ` :type "/Game/LMS_Game/Characters/Weapons/BP_Weapon_Master Object Reference"))
  ;[0.05098 0.05098 0.05098] Drop Weapon - Allows the player to drop the Weapon Currently Equipped in thier Hand
  (`/Engine/EditorBlueprintResources/StandardMacros.IsValid` `Weapon to Drop `
    (:`Is Valid`
      (`self.Drop Weapon ` `Weapon to Drop `)
      (`self.Equiping A Weapon Based on Input` "NewEnumerator4")
      (set `self.Last Known Weapon Input ` "NewEnumerator0"))))

(fn `Attach Weapon To Owner `
  (params (`Weapon ` :type "/Game/LMS_Game/Characters/Weapons/BP_Weapon_Master Object Reference") (`Holster Name ` :type Name))
  (`Actor.K2_AttachToComponent` `Weapon ` (`Character.Mesh` (`self.Character Ref `)) `Holster Name ` "SnapToTarget" "SnapToTarget" "SnapToTarget" true)
  (`/Game/LMS_Game/Characters/Weapons/BP_Weapon_Master.Set Weapon State ` (`local.Weapon `) "NewEnumerator1")
  (bind _weapon_slot_ (`self.Get Slot Based On Weapon` (`local.Weapon `)))
  (set `self.Weapon Input ` _weapon_slot_)
  (`self.Equip Event `))

(fn `Drop Weapon `
  (params (`Weapon to Drop ` :type "/Game/LMS_Game/Characters/Weapons/BP_Weapon_Master Object Reference"))
  (returns (`Dropped Weapon` :type "/Game/LMS_Game/Characters/Weapons/BP_Weapon_Master Object Reference"))
  (locals (`Weapon Slot ` :type "/Game/LMS_Game/Characters/Enums/E_Weapon_Inputs Enum" :default "NewEnumerator0"))
  (bind _weapon_to_drop_ (`local.Weapon to Drop `))
  (bind _weapon_slot_ (`self.Get Slot Based On Weapon` `Weapon to Drop `))
  (set `local.Weapon Slot ` _weapon_slot_)
  (`Actor.K2_DetachFromActor` _weapon_to_drop_ "KeepWorld" "KeepWorld" "KeepWorld")
  (`/Game/LMS_Game/Characters/Weapons/BP_Weapon_Master.Set Weapon State ` _weapon_to_drop_ "NewEnumerator0")
  (set `self.In Hand Weapon ` null)
  (switch `/Game/LMS_Game/Characters/Enums/E_Weapon_Inputs` (`local.Weapon Slot `)
    (:`NewEnumerator1`
      (set `self.Primary Holster ` null)
      (set `self.Rifle Equipped?` false))
    (:`NewEnumerator2`
      (set `self.Secondary Holster` null)
      (set `self.Rifle Equipped?` false))
    (:`NewEnumerator5`
      (set `self.Hand Gun Holster` null)
      (set `self.Hand Gun Equipped?` false))
    (:`NewEnumerator3`
      (set `self.Mellee Holster` null)
      (set `self.Mellee Equipped?` false)))
  (return _weapon_to_drop_))

(fn `Equip/Unequip`
  (params (Weapon :type "/Game/LMS_Game/Characters/Weapons/BP_Weapon_Master Object Reference") (`Want to Equip?` :type Boolean))
  (locals (`Weapon Slot` :type "/Game/LMS_Game/Characters/Enums/E_Weapon_Inputs Enum" :default "NewEnumerator0"))
  (bind (_weapon_slot_ _relative_holster_name) (`self.Get Slot Based On Weapon` Weapon))
  (set `local.Weapon Slot` _weapon_slot_)
  (`Actor.K2_AttachToComponent` (`local.Weapon`) (`Character.Mesh` (`self.Character Ref `)) (select `bool` `Want to Equip?` :`false` _relative_holster_name :`true` "InHandSocket") "SnapToTarget" "SnapToTarget" "SnapToTarget" true)
  (switch `/Game/LMS_Game/Characters/Enums/E_Weapon_Inputs` (`local.Weapon Slot`)
    (:`NewEnumerator1`
      (set `self.Rifle Equipped?` true))
    (:`NewEnumerator2`
      (set `self.Rifle Equipped?` true))
    (:`NewEnumerator5`
      (set `self.Hand Gun Equipped?` true))
    (:`NewEnumerator3`
      (set `self.Mellee Equipped?` true)))
  (if (`local.Want to Equip?`)
    (bind _output_get (set `self.In Hand Weapon ` (`local.Weapon`)))
    (`/Game/LMS_Game/Characters/Weapons/BP_Weapon_Master.Set Weapon State ` _output_get "NewEnumerator2")
    (return)
    (else
      (`/Game/LMS_Game/Characters/Weapons/BP_Weapon_Master.Set Weapon State ` (`local.Weapon`) "NewEnumerator1")
      (set `self.In Hand Weapon ` null)
      (set `self.Rifle Equipped?` false)
      (set `self.Hand Gun Equipped?` false)
      (set `self.Mellee Equipped?` false)
      (return))))

(fn `Equiping A Weapon Based on Input`
  (params (`Weapon Input` :type "/Game/LMS_Game/Characters/Enums/E_Weapon_Inputs Enum" :default "NewEnumerator0"))
  (bind _output_get (set `self.Weapon Input ` `Weapon Input`))
  (if (`self.Weapon Type Anim` _output_get)
    (`AbilitySystemComponent.TryActivateAbilityByClass` (`AbilitySystemBlueprintLibrary.GetAbilitySystemComponent` (`self.Character Ref `)) "/Game/LMS_Game/Characters/GAS/Abilities/GA_EquipWeapon.GA_EquipWeapon_C" true)
    (else
      (`self.Equip Event `)))
  (switch `/Game/LMS_Game/Characters/Enums/E_Weapon_Inputs` _output_get
    (:`NewEnumerator1`
      (set `self.Last Known Weapon Input ` "NewEnumerator1"))
    (:`NewEnumerator2`
      (set `self.Last Known Weapon Input ` "NewEnumerator2"))
    (:`NewEnumerator5`
      (set `self.Last Known Weapon Input ` "NewEnumerator5"))
    (:`NewEnumerator3`
      (set `self.Last Known Weapon Input ` "NewEnumerator3"))))

(fn `Get Slot Based On Weapon`
  (params (`Weapon ` :type "/Game/LMS_Game/Characters/Weapons/BP_Weapon_Master Object Reference"))
  (returns (`Weapon Slot ` :type "/Game/LMS_Game/Characters/Enums/E_Weapon_Inputs Enum") (`Relative Holster Name` :type Name))
  (if (and (`KismetSystemLibrary.IsValid` (`self.Primary Holster `)) (== (`local.Weapon `) (`self.Primary Holster `)))
    (return "NewEnumerator1" "Primary Holster")
    (elif (and (`KismetSystemLibrary.IsValid` (`self.Secondary Holster`)) (== (`local.Weapon `) (`self.Secondary Holster`)))
      (return "NewEnumerator2" "Secondary Holster")
      (elif (and (`KismetSystemLibrary.IsValid` (`self.Hand Gun Holster`)) (== (`local.Weapon `) (`self.Hand Gun Holster`)))
        (return "NewEnumerator5" "HandGun Holster")
        (elif (and (`KismetSystemLibrary.IsValid` (`self.Mellee Holster`)) (== (`local.Weapon `) (`self.Mellee Holster`)))
          (return "NewEnumerator3" "Mellee Holster"))))))

(fn `Get Weapons Based on Inputs`
  (params (`Weapon Input ` :type "/Game/LMS_Game/Characters/Enums/E_Weapon_Inputs Enum" :default "NewEnumerator0"))
  (returns (`Weapon ` :type "/Game/LMS_Game/Characters/Weapons/BP_Weapon_Master Object Reference"))
  (bind _primary_holster_ (`self.Primary Holster `))
  (bind _secondary_holster (`self.Secondary Holster`))
  (bind _hand_gun_holster (`self.Hand Gun Holster`))
  (bind _mellee_holster (`self.Mellee Holster`))
  (bind _in_hand_weapon_ (`self.In Hand Weapon `))
  (switch `/Game/LMS_Game/Characters/Enums/E_Weapon_Inputs` `Weapon Input `
    (:`NewEnumerator1`
      (`/Engine/EditorBlueprintResources/StandardMacros.IsValid` _primary_holster_
        (:`Is Valid`
          (return _primary_holster_))))
    (:`NewEnumerator2`
      (`/Engine/EditorBlueprintResources/StandardMacros.IsValid` _secondary_holster
        (:`Is Valid`
          (return _secondary_holster))))
    (:`NewEnumerator5`
      (`/Engine/EditorBlueprintResources/StandardMacros.IsValid` _hand_gun_holster
        (:`Is Valid`
          (return _hand_gun_holster))))
    (:`NewEnumerator3`
      (`/Engine/EditorBlueprintResources/StandardMacros.IsValid` _mellee_holster
        (:`Is Valid`
          (return _mellee_holster))))
    (:`NewEnumerator4`
      (`/Engine/EditorBlueprintResources/StandardMacros.IsValid` _in_hand_weapon_
        (:`Is Valid`
          (return _in_hand_weapon_))))))

(fn `Has Weapon Equiped?`
  (returns (`Weapon Equipped?` :type Boolean))
  (return (or (`self.Rifle Equipped?`) (`self.Hand Gun Equipped?`) (`self.Mellee Equipped?`))))

(fn `IF Get Actor References`
  (returns (Actor :type "Character Object Reference") (`Actor Camera` :type "CameraComponent Object Reference") (`Camera Boom` :type "SpringArmComponent Object Reference") (`Weapon System Component` :type "/Game/LMS_Game/Characters/Actor_Components/BPC_Weapon_System Object Reference") (`Damage System Component ` :type "/Game/LMS_Game/Characters/Actor_Components/BPC_Damage_System Object Reference"))
  (return null null null null null))

(fn `IF Get Axis Values`
  (returns (Forward :type "Float (double-precision)") (Right :type "Float (double-precision)"))
  (return 0.0 0.0))

(fn `IF Get Equipped Weapon Input `
  (returns (`Weapon Input` :type "/Game/LMS_Game/Characters/Enums/E_Weapon_Inputs Enum"))
  (return "NewEnumerator0"))

(fn `IF Get LHIK`
  (returns (LHIK :type "Transform Structure") (`Turn LHIK On?` :type Boolean)))

(fn `IF Is Aiming?`
  (returns (`Aiming?` :type Boolean))
  (return (`self.Aiming?`)))

(fn `IF Is Dead`
  (returns (`Dead?` :type Boolean))
  (return false))

(fn `IF Is Firing?`
  (returns (`Firing?` :type Boolean)))

(fn `Pick Up Weapon`
  (params (`The Weapon ` :type "/Game/LMS_Game/Characters/Weapons/BP_Weapon_Master Object Reference"))
  (locals (`Interacting Weapon ` :type "/Game/LMS_Game/Characters/Weapons/BP_Weapon_Master Object Reference"))
  (bind _output_get (set `local.Interacting Weapon ` `The Weapon `))
  ;[0.05098 0.05098 0.05098] Checks the availability of the holsters depedning on the Weapon type Itself.
  (switch `/Game/LMS_Game/Characters/Enums/E_Weapon_Types` (`.WeaponType_16_353EC415483F454D94A166BBB6421A63` (break `/Game/LMS_Game/Characters/Structures/S_Weapon_Struct` (`/Game/LMS_Game/Characters/Weapons/BP_Weapon_Master.Weapon_Structure` _output_get)))
    (:`NewEnumerator1`
      (bind _the_weapon_ (`self.Check Rifle Holster Availability ` (`local.Interacting Weapon `) :!label _label)
        (:`Full Holsters `
          ;[0.05098 0.05098 0.05098] Since full holsters Output means a slot just became empty since a weapon was dropped, the function is called again , but this time directly attaching the weapon to the actor due to another free holster being available
          (`self.Pick Up Weapon` (`local.Interacting Weapon `)))
        (:`Secondary Holster Empty `
          (bind _output_get_2 (set `self.Secondary Holster` _the_weapon_))
          (`self.Attach Weapon To Owner ` _output_get_2 (`self.Empty Holster `))
          (set `self.Last Known Weapon Input ` "NewEnumerator2"))
        (:`Primary Holster Empty `
          (bind _output_get_3 (set `self.Primary Holster ` _the_weapon_))
          (`self.Attach Weapon To Owner ` _output_get_3 (`self.Empty Holster `))
          (set `self.Last Known Weapon Input ` "NewEnumerator1"))))
    (:`NewEnumerator2`
      (bind _the_weapon (`self.Check HandGun Holster Availabilty ` (`local.Interacting Weapon `) :!label _label_2)
        (:`HandGun Holster Full`
          (`self.Pick Up Weapon` (`local.Interacting Weapon `)))
        (:`HandGun Holster Empty`
          (bind _output_get_4 (set `self.Hand Gun Holster` _the_weapon))
          (`self.Attach Weapon To Owner ` _output_get_4 (`self.Empty Holster `))
          (set `self.Last Known Weapon Input ` "NewEnumerator5"))))
    (:`NewEnumerator3`
      (goto _label_2))
    (:`NewEnumerator4`
      (goto _label))
    (:`NewEnumerator5`
      (goto _label))
    (:`NewEnumerator6`
      (bind _the_weapon_2 (`self.Check Mellee Holster Availabilty ` (`local.Interacting Weapon `))
        (:`Mellee Holster Full`
          (`self.Pick Up Weapon` (`local.Interacting Weapon `)))
        (:`Mellee Holster Empty`
          (bind _output_get_5 (set `self.Mellee Holster` _the_weapon_2))
          (`self.Attach Weapon To Owner ` _output_get_5 (`self.Empty Holster `))
          (set `self.Last Known Weapon Input ` "NewEnumerator3"))))))

(fn `Quik Equip Weapon `
  (bind _last_known_weapon_input_ (`self.Last Known Weapon Input `))
  (`/Engine/EditorBlueprintResources/StandardMacros.IsValid` (`self.Get Weapons Based on Inputs` _last_known_weapon_input_)
    (:`Is Valid`
      (bind _output_get (set `self.Weapon Input ` _last_known_weapon_input_))
      (`self.Equip Event `)
      (`KismetSystemLibrary.PrintString` (`|GetEnumeratorNameAsString` _output_get)))))

(fn `Set Owner Mode By Enum `
  (params (`Owner Mode` :type "/Game/LMS_Game/Characters/Enums/E_Owner_Mode Enum" :default "NewEnumerator0"))
  (bind _output_get (set `self. Owner Mode (Combat/Non-Combat)` `Owner Mode`))
  (switch `/Game/LMS_Game/Characters/Enums/E_Owner_Mode` _output_get
    (:`NewEnumerator1`
      (bind _character_movement (`self.Character Movement`)
        (:`then`
          (set `CharacterMovementComponent.MaxWalkSpeed` (`self.Non Combat Walk Speed `) _character_movement)
          (set `CharacterMovementComponent.RotationRate` (struct :`Yaw` 500.0) _character_movement)
          (set `CharacterMovementComponent.bOrientRotationToMovement` true _character_movement)
          (set `CharacterMovementComponent.bUseControllerDesiredRotation` false _character_movement))
        (:`else`)))
    (:`NewEnumerator2`
      (bind _character_movement_2 (`self.Character Movement`)
        (:`then`
          (set `CharacterMovementComponent.MaxWalkSpeed` (`self.Combat Walk Speed`) _character_movement_2)
          (set `CharacterMovementComponent.RotationRate` (struct :`Yaw` 5000.0) _character_movement_2)
          (set `CharacterMovementComponent.bOrientRotationToMovement` false _character_movement_2)
          (set `CharacterMovementComponent.bUseControllerDesiredRotation` true _character_movement_2))
        (:`else`)))))

(fn `Swap Weapon`
  (params (Weapon :type "/Game/LMS_Game/Characters/Weapons/BP_Weapon_Master Object Reference"))
  (locals (`Next Weapon Slot ` :type "/Game/LMS_Game/Characters/Enums/E_Weapon_Inputs Enum" :default "NewEnumerator0") (`Next Weapon Holster` :type Name :default "None") (`In Hand Slot ` :type "/Game/LMS_Game/Characters/Enums/E_Weapon_Inputs Enum" :default "NewEnumerator0") (`InHand Holster` :type Name :default "None"))
  (bind (_weapon_slot_ _relative_holster_name) (`self.Get Slot Based On Weapon` Weapon))
  (set `local.Next Weapon Slot ` _weapon_slot_)
  (set `local.Next Weapon Holster` _relative_holster_name)
  (bind (_weapon_slot__2 _relative_holster_name_2) (`self.Get Slot Based On Weapon` (`self.In Hand Weapon `)))
  (set `local.In Hand Slot ` _weapon_slot__2)
  (bind _output_get (set `local.InHand Holster` _relative_holster_name_2))
  (`Actor.K2_AttachToComponent` (`self.In Hand Weapon `) (`Character.Mesh` (`self.Character Ref `)) _output_get "SnapToTarget" "SnapToTarget" "SnapToTarget" true)
  (`/Game/LMS_Game/Characters/Weapons/BP_Weapon_Master.Set Weapon State ` (`self.In Hand Weapon `) "NewEnumerator1")
  (set `self.In Hand Weapon ` null)
  (set `self.Rifle Equipped?` false)
  (set `self.Mellee Equipped?` false)
  (set `self.Hand Gun Equipped?` false)
  (`self.Equip/Unequip` (`local.Weapon`) true))

(fn `Weapon Type Anim`
  (params (E_Weapon :type "/Game/LMS_Game/Characters/Enums/E_Weapon_Inputs Enum" :default "NewEnumerator0"))
  (returns (`Can Animate` :type Boolean))
  (bind _in_hand_weapon_ (`self.In Hand Weapon `))
  (switch `/Game/LMS_Game/Characters/Enums/E_Weapon_Inputs` E_Weapon
    (:`NewEnumerator1`
      (`/Engine/EditorBlueprintResources/StandardMacros.IsValid` (`self.Primary Holster `)
        (:`Is Valid`
          _)
        (:`Is Not Valid`
          (set `self.Weapon Input ` "NewEnumerator0" :!label _label)
          (return false))))
    (:`NewEnumerator2`
      (`/Engine/EditorBlueprintResources/StandardMacros.IsValid` (`self.Secondary Holster`)
        (:`Is Valid`
          _)
        (:`Is Not Valid`
          (goto _label))))
    (:`NewEnumerator5`
      (`/Engine/EditorBlueprintResources/StandardMacros.IsValid` (`self.Hand Gun Holster`)
        (:`Is Valid`
          _)
        (:`Is Not Valid`
          (goto _label))))
    (:`NewEnumerator3`
      (`/Engine/EditorBlueprintResources/StandardMacros.IsValid` (`self.Mellee Holster`)
        (:`Is Valid`
          _)
        (:`Is Not Valid`
          (goto _label))))
    (:`NewEnumerator4`
      (`/Engine/EditorBlueprintResources/StandardMacros.IsValid` (`self.In Hand Weapon `)
        (:`Is Valid`
          (set `self.Weapon Input ` "NewEnumerator4")
          (return false)))))
  (`/Engine/EditorBlueprintResources/StandardMacros.IsValid` _in_hand_weapon_
    (:`Is Valid`
      (bind _weapon_slot_ (`self.Get Slot Based On Weapon` _in_hand_weapon_))
      (if (`|EnumEquality` _weapon_slot_ (`self.Weapon Input `))
        (set `self.Weapon Input ` "NewEnumerator0")
        (return false)
        (else
          _)))
    (:`Is Not Valid`
      _))
  (set `self.Weapon Input ` (`self.Weapon Input `))
  (return true))