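; Actor component that tracks health for its owner and handles healing and incoming damage.
; TakeDamage uses a Can Be Damaged macro to block, apply or ignore hits based on death, invincibility and blocking state.
; Dispatchers report blocks with parry eligibility, deaths, and damage responses for interruptible or force-interrupt hits.
; Heal clamps health to the maximum and only works while alive.
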(fn `Heal`
  (params (Amount :type "Float (double-precision)"))
  (returns (`New Health` :type "Float (double-precision)"))
  (if (not (`self.IsDead?`))
    (bind _output_get (set `self.Health` (`KismetMathLibrary.FClamp` (+ (`self.Health`) Amount) 0.0 (`self.Max Health`))))
    (return _output_get)))

(fn `Take Damage`
  (params (`Damage Info` :type "/Game/LMS_Game/Characters/Structures/S_DamageInfo Structure") (`Damage Causer` :type "Actor Object Reference"))
  (returns (`Was Damaged?` :type Boolean))
  (bind (_damageamount _damagetype _damageresponse _shoulddamageinvincible _canbeblocked _canbeparried _shouldforceinterupt _iscriticaldamage_ _hitresult) (break `/Game/LMS_Game/Characters/Structures/S_DamageInfo` `Damage Info`))
  (`self.Can Be Damaged` _shoulddamageinvincible _canbeblocked
    (:`Block Damage`
      (`KismetSystemLibrary.PrintString` "Blocked")
      (`self.On Blocked` _canbeparried)
      (return false))
    (:`Do Damage`
      (bind _output_get (set `self.Health` (- (`self.Health`) _damageamount)))
      (if (<= _output_get 0.0)
        (set `self.IsDead?` true)
        (`self.On Death` (`local.Damage Causer`) _hitresult)
        (return true)
        (elif (or (`self.Is Interuptable?`) _shouldforceinterupt)
          (set `self.Is Critical Damage` _iscriticaldamage_)
          (`self.On Damage Response` _damageresponse (`local.Damage Causer`) _hitresult)
          (return true))))
    (:`No Damage`
      (return false))))