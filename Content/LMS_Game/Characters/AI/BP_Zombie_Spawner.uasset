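; Zombie wave spawner that spawns BP_LMS_Zombie_Character actors whenever BP_LMS_GameMode signals the next wave.
; On BeginPlay it binds SpawnZombies to that signal, which waits briefly before spawning the batch.
; Zombies appear at random navmesh-reachable points within the Sphere radius, with random yaw and collision-adjusted placement.
; Each wave raises SpawnIncrement and adds it to ZombiesSpawned, so batches grow at an accelerating rate, then increments the GameMode's ZombieWave.
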(event `self.ReceiveBeginPlay`
  (bind _asbp_lms_game_mode (cast `/Game/LMS_Game/Characters/Character_Logic/BP_LMS_GameMode` (`GameplayStatics.GetGameMode`)))
  (add `/Game/LMS_Game/Characters/Character_Logic/BP_LMS_GameMode.Spawn Next Wave` _asbp_lms_game_mode (delegate `Spawn Zombies`)))

(event `Spawn Zombies`
  (`KismetSystemLibrary.Delay` 3.0)
  (for _ (range (`self.Zombies Spawned`))
    (`|SpawnActorFromClass` "/Game/LMS_Game/Characters/Character_Logic/BP_LMS_Zombie_Character.BP_LMS_Zombie_Character_C" (`KismetMathLibrary.MakeTransform` (`NavigationSystemV1.K2_GetRandomReachablePointInRadius` (.location (`self.GetTransform`)) (`SphereComponent.SphereRadius` (`self.Sphere`)) null null) (`KismetMathLibrary.MakeRotator` (.roll (.rotation (`self.GetTransform`))) (.pitch (.rotation (`self.GetTransform`))) (`KismetMathLibrary.RandomFloatInRange` 0.0 360.0))) "AdjustIfPossibleButAlwaysSpawn" "OverrideRootScale" null null))
  (`/Engine/EditorBlueprintResources/StandardMacros.IncrementInt` (`self.Spawn Increment`)
    (:`  `
      (set `self.Zombies Spawned` (+ (`self.Zombies Spawned`) (`self.Spawn Increment`)))
      (bind _asbp_lms_game_mode (cast `/Game/LMS_Game/Characters/Character_Logic/BP_LMS_GameMode` (`GameplayStatics.GetGameMode`)))
      (`/Engine/EditorBlueprintResources/StandardMacros.IncrementInt` (`/Game/LMS_Game/Characters/Character_Logic/BP_LMS_GameMode.Zombie Wave` _asbp_lms_game_mode)))))

(fn `UserConstructionScript`)